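; Training grounds dummy character that chases the player's Tiki and stuns it with a bat hit.
; StartChase, gated by a DoOnce that StopChase resets, moves the AI to the player and plays the attack montage on arrival.
; The montage's "Start" notify applies stun damage to the player directly, without a hit trace.
; Inherited stun events halt the dummy's movement, then restore its walk speed afterwards.
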(event `StartChase`
  (`/Engine/EditorBlueprintResources/StandardMacros.DoOnce` false :!label _label
    (:`Completed`
      (bind _asbp_tiki (cast `/Game/Core/Blueprints/TikiCharacter/Blueprint/BP_Tiki` (`GameplayStatics.GetPlayerCharacter` 0)))
      (`|AIMoveTo` self (0.0 0.0 0.0) _asbp_tiki 10.0
        (:`OnSuccess`
          (`self.HeavyAttackStarted`))))))

(event `self.ReceiveBeginPlay`
  ;[1 1 1] Event BeginPlay
  (`parent.ReceiveBeginPlay`)
  (add `self.OnUnStunned` (delegate `ResetOnUnStunned`))
  (add `self.OnStunned` (delegate `Stop`)))

(event `StopChase`
  (goto _label :!via `Reset`))

(event `ResetOnUnStunned`
  ;[1 1 1] Event BeginPlay
  (set `CharacterMovementComponent.MaxWalkSpeed` (`self.fBonkerWalkSpeed`) (`self.CharacterMovement`)))

(event `Stop`
  ;[1 1 1] Event BeginPlay
  (`NavMovementComponent.StopActiveMovement` (`self.CharacterMovement`)))

(event `HeavyAttackStarted`
  ;[0 1 0.8588] HeavyAttack
  (bind _notifyname (`|PlayMontage` (`self.Mesh`) "/Game/Assets/TikiCharacter/Animations/Bonkerman/AM_BatHit.AM_BatHit")
    (:`OnBlendOut`
      (set `self.eState` "NewEnumerator0"))
    (:`OnNotifyBegin`
      (if (== _notifyname "Start")
        (bind _asbp_tiki (cast `/Game/Core/Blueprints/TikiCharacter/Blueprint/BP_Tiki` (`GameplayStatics.GetPlayerCharacter` 0)))
        (`/Engine/EditorBlueprintResources/StandardMacros.IsValid` _asbp_tiki
          (:`Is Valid`
            (`GameplayStatics.ApplyDamage` _asbp_tiki 1.0 null self "/Game/Core/Data/DamageTypes/DT_Stun.DT_Stun_C")))))))

(fn `HeavyVFX`
  (params (SystemTemplate :type "NiagaraSystem Object Reference") (Location :type "Vector Structure"))
  (`NiagaraFunctionLibrary.SpawnSystemAtLocation` SystemTemplate Location)
  (`GameplayStatics.SpawnSoundAtLocation` "/Game/Assets/SFX/MS_FootSteps.MS_FootSteps" (`self.K2_GetActorLocation`) (struct) 1.0 1.0 0.0 null null))

(fn `UserConstructionScript`
  (set `self.eCharacterClass` "NewEnumerator1")
  (`parent.UserConstructionScript`))