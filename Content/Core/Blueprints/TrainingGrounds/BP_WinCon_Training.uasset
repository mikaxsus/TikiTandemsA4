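; Training Grounds variant of the win-condition totem, used to teach players its rotating fists and wings through scripted examples and quest steps.
; RotateTotem extends the parent's rotation, counting three turns in quests 10 and 11 to trigger W_TotemExplanation intros and toggle the fist lock.
; A looping timer then watches the wings' yaw to start the arena outro.
; Highlight functions use custom depth stencil values to emphasize totem parts.
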(event `FistsExample`
  (`/Engine/EditorBlueprintResources/StandardMacros.DoOnce` false
    (:`Completed`
      (`self.RotateTotem` "NewEnumerator0" 1.5 "NewEnumerator3"))))

(event `WingsExample`
  (`/Engine/EditorBlueprintResources/StandardMacros.DoOnce` false
    (:`Completed`
      (`self.RotateTotem` "NewEnumerator0" 1.5 "NewEnumerator1"))))

(event `StartWingsTraining`
  (`/Engine/EditorBlueprintResources/StandardMacros.DoOnce` false
    (:`Completed`
      (set `self.bAreFistsLocked?` true)
      (`self.RotateTotem` "NewEnumerator1" 1.0 "NewEnumerator1"))))

(event `self.RotateTotem`
  (params (Rotation :type "/Game/Core/Data/Enums/E_TotemRotation Enum" :default "NewEnumerator0") (TurnAmount :type "Float (double-precision)") (TotemPartHit :type "/Game/Core/Data/Enums/E_TotemPart Enum" :default "NewEnumerator0"))
  (`parent.RotateTotem` Rotation TurnAmount TotemPartHit)
  (if (== (`self.CurrentQuest`) "10")
    (bind _counter (`/Engine/EditorBlueprintResources/StandardMacros.Do N` 3)
      (:`Exit`
        (if (== _counter 3)
          (set `self.bAreFistsLocked?` false)
          (bind _foundwidgets (`WidgetBlueprintLibrary.GetAllWidgetsOfClass` "/Game/Core/Widgets/TrainingGrounds/ExplanationWidgets/W_TotemExplanation.W_TotemExplanation_C"))
          (`/Game/Core/Widgets/TrainingGrounds/ExplanationWidgets/W_TotemExplanation.StartFistsIntro` (`|GetArrayItem` _foundwidgets)))))
    (elif (== (`self.CurrentQuest`) "11")
      (bind _counter_2 (`/Engine/EditorBlueprintResources/StandardMacros.Do N` 3)
        (:`Exit`
          (if (== _counter_2 3)
            (bind _foundwidgets_2 (`WidgetBlueprintLibrary.GetAllWidgetsOfClass` "/Game/Core/Widgets/TrainingGrounds/ExplanationWidgets/W_TotemExplanation.W_TotemExplanation_C"))
            (`/Game/Core/Widgets/TrainingGrounds/ExplanationWidgets/W_TotemExplanation.StartWinIntro` (`|GetArrayItem` _foundwidgets_2))
            (bind _returnvalue (`KismetSystemLibrary.K2_SetTimerDelegate` (delegate `CheckEndGame`) 0.01 true))))))))

(event `CheckEndGame`
  (bind (_relativerotation_roll _relativerotation_pitch _relativerotation_yaw) (`KismetMathLibrary.BreakRotator` (`SceneComponent.RelativeRotation` (`self.WingsBase`))))
  (if (<= _relativerotation_yaw -170.0)
    (`KismetSystemLibrary.K2_ClearAndInvalidateTimerHandle` (stale `self.RotateTotem` _returnvalue))
    (bind _foundwidgets (`WidgetBlueprintLibrary.GetAllWidgetsOfClass` "/Game/Core/Widgets/TrainingGrounds/ExplanationWidgets/W_TotemExplanation.W_TotemExplanation_C"))
    (`/Game/Core/Widgets/TrainingGrounds/ExplanationWidgets/W_TotemExplanation.StartArenaOutro` (`|GetArrayItem` _foundwidgets))))

(fn `HighlightFists`
  (`PrimitiveComponent.SetCustomDepthStencilValue` (`self.WingsBase`) 0)
  (`PrimitiveComponent.SetCustomDepthStencilValue` (`self.L_Wing`) 0)
  (`PrimitiveComponent.SetCustomDepthStencilValue` (`self.R_Wing`) 0)
  (`PrimitiveComponent.SetCustomDepthStencilValue` (`self.HornsTotem`) 0)
  (`PrimitiveComponent.SetCustomDepthStencilValue` (`self.TotemBase`) 0)
  (`PrimitiveComponent.SetCustomDepthStencilValue` (`self.R_Fist`) 1)
  (`PrimitiveComponent.SetCustomDepthStencilValue` (`self.L_Fist`) 1)
  (`PrimitiveComponent.SetCustomDepthStencilValue` (`self.FistsBase`) 1))

(fn `HighlightTotem`
  (params (Value :type Integer))
  (`PrimitiveComponent.SetCustomDepthStencilValue` (`self.FistsBase`) Value)
  (`PrimitiveComponent.SetCustomDepthStencilValue` (`self.R_Fist`) Value)
  (`PrimitiveComponent.SetCustomDepthStencilValue` (`self.L_Fist`) Value)
  (`PrimitiveComponent.SetCustomDepthStencilValue` (`self.WingsBase`) Value)
  (`PrimitiveComponent.SetCustomDepthStencilValue` (`self.L_Wing`) Value)
  (`PrimitiveComponent.SetCustomDepthStencilValue` (`self.R_Wing`) Value)
  (`PrimitiveComponent.SetCustomDepthStencilValue` (`self.HornsTotem`) Value)
  (`PrimitiveComponent.SetCustomDepthStencilValue` (`self.TotemBase`) Value))

(fn `HighlightWings`
  (`PrimitiveComponent.SetCustomDepthStencilValue` (`self.WingsBase`) 1)
  (`PrimitiveComponent.SetCustomDepthStencilValue` (`self.L_Wing`) 1)
  (`PrimitiveComponent.SetCustomDepthStencilValue` (`self.R_Wing`) 1)
  (`PrimitiveComponent.SetCustomDepthStencilValue` (`self.HornsTotem`) 1)
  (`PrimitiveComponent.SetCustomDepthStencilValue` (`self.TotemBase`) 1)
  (`PrimitiveComponent.SetCustomDepthStencilValue` (`self.R_Fist`) 0)
  (`PrimitiveComponent.SetCustomDepthStencilValue` (`self.L_Fist`) 0)
  (`PrimitiveComponent.SetCustomDepthStencilValue` (`self.FistsBase`) 0))

(fn `UserConstructionScript`)