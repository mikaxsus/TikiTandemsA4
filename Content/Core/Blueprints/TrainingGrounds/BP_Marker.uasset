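; BP_Marker is a Training Grounds trigger that reacts when a BP_Tiki overlaps its Collision component.
; With IsRespawn set, it acts as a checkpoint, writing the collision's world transform to TSpawnPos on the BPC_TrainingGrounds player controller.
; Otherwise it destroys itself on overlap unless IsReusable is set, with no other effect.
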(event `self.Collision.OnComponentBeginOverlap`
  (params (OverlappedComponent :type "PrimitiveComponent Object Reference") (OtherActor :type "Actor Object Reference") (OtherComp :type "PrimitiveComponent Object Reference") (OtherBodyIndex :type Integer) (bFromSweep :type Boolean) (SweepResult :type "HitResult Structure (by ref)"))
  (cast `/Game/Core/Blueprints/TikiCharacter/Blueprint/BP_Tiki` OtherActor)
  (if (`self.bIsRespawn?`)
    (bind _asbpc_training_grounds (cast `/Game/Core/Blueprints/Input/Controllers/BPC_TrainingGrounds` (`GameplayStatics.GetPlayerController` 0)))
    (set `/Game/Core/Blueprints/Input/Controllers/BPC_TrainingGrounds.tSpawnPos` (`SceneComponent.K2_GetComponentToWorld` (`self.Collision`)) _asbpc_training_grounds)
    (else
      (if (not (`self.bIsReusable?`))
        (`self.K2_DestroyActor`))
      (if true
        _))))

(fn `UserConstructionScript`)