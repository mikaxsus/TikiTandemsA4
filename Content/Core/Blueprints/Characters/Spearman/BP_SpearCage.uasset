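; BP_SpearCage is a spawned Spearman hazard that raises a cage of spears and retracts it after a short delay.
; On BeginPlay it plays an impact sound and camera shake, then a FlipFlop plays and later reverses a timeline driving the SpearBase's vertical position.
; Any overlapping actor other than the instigator takes stun-type damage and triggers another camera shake.
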(event `self.ReceiveBeginPlay`
  (`GameplayStatics.SpawnSound2D` "/Game/Assets/SFX/MS_SpearCageImpact.MS_SpearCageImpact" 1.0 1.0 0.0 null)
  (`self.SpearAnimation`)
  (`GameplayStatics.PlayWorldCameraShake` "/Game/Core/Cinematics/CameraShake/BP_SpearCage_CS.BP_SpearCage_CS_C" (`self.K2_GetActorLocation`))
  (`KismetSystemLibrary.Delay` 3.0)
  (`self.SpearAnimation`))

(event `SpearAnimation`
  (bind _spearbase (`self.SpearBase`))
  (bind (_relativelocation_x _relativelocation_y) (`KismetMathLibrary.BreakVector` (`SceneComponent.RelativeLocation` _spearbase)))
  (`/Engine/EditorBlueprintResources/StandardMacros.FlipFlop`
    (:`A`
      (bind (_direction _zmovement) (`Timeline|SpearCageAnimation` :!label _label)
        (:`Update`
          (`SceneComponent.K2_SetRelativeLocation` _spearbase (`KismetMathLibrary.MakeVector` _relativelocation_x _relativelocation_y _zmovement) false false))))
    (:`B`
      (goto _label :!via `Reverse`))))

(event `self.Collision.OnComponentBeginOverlap`
  (params (OverlappedComponent :type "PrimitiveComponent Object Reference") (OtherActor :type "Actor Object Reference") (OtherComp :type "PrimitiveComponent Object Reference") (OtherBodyIndex :type Integer) (bFromSweep :type Boolean) (SweepResult :type "HitResult Structure (by ref)"))
  (bind _instigator (`self.Instigator`))
  (if (!= OtherActor _instigator)
    (`GameplayStatics.ApplyDamage` OtherActor 1.0 null _instigator "/Game/Core/Data/DamageTypes/DT_Stun.DT_Stun_C")
    (`GameplayStatics.PlayWorldCameraShake` "/Game/Core/Cinematics/CameraShake/BP_SpearCage_CS.BP_SpearCage_CS_C" (`self.K2_GetActorLocation`))))

(fn `UserConstructionScript`)