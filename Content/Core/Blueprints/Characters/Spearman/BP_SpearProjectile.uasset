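; Spearman projectile that damages Tiki players and BP_WinCon totems, ignoring its Instigator.
; A normal player hit applies launch and half-strength stun damage, then destroys the spear; a special hit spawns a BP_SpearCage at the player instead.
; Other hits remove collision, and totem hits also record the struck part, deal damage and stick the spear to it.
; Hit effects go through server/multicast events, where the special spear is also destroyed.
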(event `SR_NiagaraVFXPlayer`
  (params (SystemTemplate :type "NiagaraSystem Object Reference") (Location :type "Vector Structure") (Condition :type Boolean))
  (`self.MC_NiagaraVFXPlayer` SystemTemplate Location Condition))

(event `self.Collision.OnComponentBeginOverlap`
  (params (OverlappedComponent :type "PrimitiveComponent Object Reference") (OtherActor :type "Actor Object Reference") (OtherComp :type "PrimitiveComponent Object Reference") (OtherBodyIndex :type Integer) (bFromSweep :type Boolean) (SweepResult :type "HitResult Structure (by ref)"))
  (bind _returnvalue (`self.K2_GetActorLocation`))
  (bind _returnvalue_2 (`self.K2_GetActorLocation`))
  (bind _bisspecial_ (`self.bIsSpecial?`))
  (if (!= OtherActor (`self.Instigator`))
    (cast `/Game/Core/Blueprints/TikiCharacter/Blueprint/BP_Tiki` OtherActor
      (:`then`
        (if (`self.bIsSpecial?`)
          (`self.IfHitPlayerSpecial` OtherActor)
          (else
            (`self.IfHitPlayer` OtherActor)))
        (if (`KismetSystemLibrary.IsServer`)
          (`self.SR_NiagaraVFXPlayer` "/Game/Assets/VFX/Flipbook_VFX/Shared/Particles/Blood/NS_SpearHitPlayer.NS_SpearHitPlayer" _returnvalue _bisspecial_)
          (else
            (`self.MC_NiagaraVFXPlayer` "/Game/Assets/VFX/Flipbook_VFX/Shared/Particles/Blood/NS_SpearHitPlayer.NS_SpearHitPlayer" _returnvalue _bisspecial_))))
      (:`CastFailed`
        (`self.IfHitTotem` OtherActor OtherComp)
        (if (`KismetSystemLibrary.IsServer`)
          (`self.SR_NiagaraVFXTotem` "/Game/Assets/VFX/Flipbook_VFX/Shared/Particles/Dust/NS_DustHit.NS_DustHit" _returnvalue_2)
          (else
            (`self.MC_NiagaraVFXTotem` "/Game/Assets/VFX/Flipbook_VFX/Shared/Particles/Dust/NS_DustHit.NS_DustHit" _returnvalue_2)))))))

(event `MC_NiagaraVFXPlayer`
  (params (SystemTemplate :type "NiagaraSystem Object Reference") (Location :type "Vector Structure") (Condition :type Boolean))
  (`NiagaraFunctionLibrary.SpawnSystemAtLocation` SystemTemplate Location)
  (if Condition
    (`self.K2_DestroyActor`)
    (`GameplayStatics.PlaySoundAtLocation` "/Game/Assets/SFX/MS_FootSteps.MS_FootSteps" (`self.K2_GetActorLocation`) (struct) 1.0 1.0 0.0 null null null null :!label _label)))

(event `SR_NiagaraVFXTotem`
  (params (SystemTemplate :type "NiagaraSystem Object Reference") (Location :type "Vector Structure"))
  (`self.MC_NiagaraVFXTotem` SystemTemplate Location))

(event `MC_NiagaraVFXTotem`
  (params (SystemTemplate :type "NiagaraSystem Object Reference") (Location :type "Vector Structure"))
  (`NiagaraFunctionLibrary.SpawnSystemAtLocation` SystemTemplate Location)
  (goto _label))

(fn `IfHitPlayer`
  (params (Object :type "Object Object Reference"))
  (bind _flaunchstrength (`self.fLaunchStrength`))
  (bind _instigator (`self.Instigator`))
  (bind _asbp_tiki (cast `/Game/Core/Blueprints/TikiCharacter/Blueprint/BP_Tiki` Object))
  (`GameplayStatics.ApplyDamage` _asbp_tiki _flaunchstrength null _instigator "/Game/Core/Data/DamageTypes/DT_Launch.DT_Launch_C")
  (`GameplayStatics.ApplyDamage` _asbp_tiki (/ _flaunchstrength 2.0) null _instigator "/Game/Core/Data/DamageTypes/DT_Stun.DT_Stun_C")
  (`self.K2_DestroyActor`))

(fn `IfHitPlayerSpecial`
  (params (Object :type "Object Object Reference"))
  (bind _asbp_tiki (cast `/Game/Core/Blueprints/TikiCharacter/Blueprint/BP_Tiki` Object))
  (bind _returnvalue (`self.GetTransform` _asbp_tiki))
  (`|SpawnActorFromClass` "/Game/Core/Blueprints/Characters/Spearman/BP_SpearCage.BP_SpearCage_C" (`KismetMathLibrary.MakeTransform` (`KismetMathLibrary.MakeVector` (.x (.location _returnvalue)) (.y (.location _returnvalue)) 170.0)) "AlwaysSpawn" "MultiplyWithRoot" null null))

(fn `IfHitTotem`
  (params (OtherActor :type "Object Object Reference") (OtherComponent :type "PrimitiveComponent Object Reference"))
  (bind _collision (`self.Collision`))
  (bind _projectilemovement (`self.ProjectileMovement`))
  (`/Engine/EditorBlueprintResources/StandardMacros.IsValid` _collision
    (:`Is Valid`
      (`ActorComponent.K2_DestroyComponent` _collision))
    (:`Is Not Valid`
      _))
  (bind _asbp_win_con (cast `/Game/Core/Blueprints/WinCondition/BP_WinCon` OtherActor))
  (set `/Game/Core/Blueprints/WinCondition/BP_WinCon.HitTotemPart` OtherComponent _asbp_win_con)
  (set `/Game/Core/Blueprints/WinCondition/BP_WinCon.vHitLocation` (`self.K2_GetActorLocation`) _asbp_win_con)
  (`/Engine/EditorBlueprintResources/StandardMacros.DoOnce` false
    (:`Completed`
      (`GameplayStatics.ApplyDamage` _asbp_win_con (`self.fLaunchStrength`) null (`self.Instigator`))
      (`/Engine/EditorBlueprintResources/StandardMacros.IsValid` _projectilemovement
        (:`Is Valid`
          (`ActorComponent.K2_DestroyComponent` _projectilemovement)
          (`SceneComponent.K2_AttachToComponent` (`self.Spear`) OtherComponent "None" "KeepWorld" "KeepWorld" "KeepRelative" true))))))

(fn `UserConstructionScript`)