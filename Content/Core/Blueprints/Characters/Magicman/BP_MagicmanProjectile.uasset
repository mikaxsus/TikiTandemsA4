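; Skull projectile fired by Magicman, with launch speed scaled by the shooter's clamped charge value.
; A Tiki entering HomingRange turns on strong homing toward the last non-instigator Tiki found in the level, not necessarily the overlapping one.
; Collision overlaps apply charge-scaled stun damage to Tikis and spawn hit VFX.
; The projectile then drops movement and homing, plays a sound and leaves the skull simulating physics.
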(event `self.ReceiveBeginPlay`
  (bind _asbp_magicman (cast `/Game/Core/Blueprints/Characters/Magicman/BP_Magicman` (`self.Instigator`)))
  (bind _output_get (set `self.fLaunchStrength` (`KismetMathLibrary.FClamp` (`/Game/Core/Blueprints/TikiCharacter/Blueprint/BP_Tiki.fChargebarValue` _asbp_magicman) 0.3 (`/Game/Core/Blueprints/Characters/Magicman/BP_Magicman.fMaxChargeTime` _asbp_magicman))))
  (`ProjectileMovementComponent.SetVelocityInLocalSpace` (`self.ProjectileMovement`) (* (`self.vBaseVelocity`) _output_get)))

(event `self.Collision.OnComponentBeginOverlap`
  (params (OverlappedComponent :type "PrimitiveComponent Object Reference") (OtherActor :type "Actor Object Reference") (OtherComp :type "PrimitiveComponent Object Reference") (OtherBodyIndex :type Integer) (bFromSweep :type Boolean) (SweepResult :type "HitResult Structure (by ref)"))
  (if (and (!= OtherActor (`self.Instigator`)) (!= OtherComp (`self.HomingRange`)))
    (`|ExecutionSequence`
      (:`then_0`
        (`self.IfPlayerIsHit` OtherActor)
        (`NiagaraFunctionLibrary.SpawnSystemAtLocation` "/Game/Assets/VFX/Flipbook_VFX/Shared/Particles/Lightning/NS_SkullHit.NS_SkullHit" (`self.K2_GetActorLocation`)))
      (:`then_1`
        (`self.IfProjectileIsHit`)))))

(event `self.HomingRange.OnComponentBeginOverlap`
  (params (OverlappedComponent :type "PrimitiveComponent Object Reference") (OtherActor :type "Actor Object Reference") (OtherComp :type "PrimitiveComponent Object Reference") (OtherBodyIndex :type Integer) (bFromSweep :type Boolean) (SweepResult :type "HitResult Structure (by ref)"))
  (bind _projectilemovement (`self.ProjectileMovement`))
  (if (!= OtherActor (`self.Instigator`))
    (cast `/Game/Core/Blueprints/TikiCharacter/Blueprint/BP_Tiki` OtherActor)
    (`self.FindHomingTarget`)
    (set `ProjectileMovementComponent.bIsHomingProjectile` true _projectilemovement)
    (set `ProjectileMovementComponent.HomingAccelerationMagnitude` 30000.0 _projectilemovement)))

(fn `FindHomingTarget`
  (bind _outactors (`GameplayStatics.GetAllActorsOfClass` "/Game/Core/Blueprints/TikiCharacter/Blueprint/BP_Tiki.BP_Tiki_C"))
  (for _array_element _outactors
    (if (!= _array_element (`self.Instigator`))
      (set `ProjectileMovementComponent.HomingTargetComponent` (`Actor.RootComponent` _array_element) (`self.ProjectileMovement`)))))

(fn `IfPlayerIsHit`
  (params (PlayerHit :type "Actor Object Reference"))
  (bind _asbp_tiki (cast `/Game/Core/Blueprints/TikiCharacter/Blueprint/BP_Tiki` PlayerHit))
  (`GameplayStatics.ApplyDamage` _asbp_tiki (`KismetMathLibrary.FClamp` (`self.fLaunchStrength`) 0.3) null (`self.Instigator`) "/Game/Core/Data/DamageTypes/DT_Stun.DT_Stun_C"))

(fn `IfProjectileIsHit`
  (bind _projectilemovement (`self.ProjectileMovement`))
  (bind _skull (`self.Skull`))
  (`/Engine/EditorBlueprintResources/StandardMacros.IsValid` _projectilemovement
    (:`Is Valid`
      (`ActorComponent.K2_DestroyComponent` _projectilemovement)
      (`PrimitiveComponent.SetCollisionEnabled` _skull "PhysicsOnly")
      (`PrimitiveComponent.SetSimulatePhysics` _skull true)
      (`ActorComponent.K2_DestroyComponent` (`self.HomingRange`))
      (`GameplayStatics.PlaySoundAtLocation` "/Game/Assets/SFX/MS_ShootBasic_MM.MS_ShootBasic_MM" (`self.K2_GetActorLocation`) (struct) 1.0 1.0 0.0 null null null null))))

(fn `UserConstructionScript`)