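; Networked preview character for two-player character selection, showing Spearman, Bonkerman or Magicman with red or blue player overlay by actor tag.
; RepNotify on the current character swaps anim class, modular part visibility and world title image.
; Unavailable characters set a custom-depth stencil and block locking.
; Server/multicast events sync flip, lock toggle and stencil; lock and face-off play per-character montages, the latter leading to the loading screen.
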(event `self.ReceiveBeginPlay`
  ;[1 1 1] Event BeginPlay
  (`parent.ReceiveBeginPlay`)
  (`self.SetCharacterMeshArrays`)
  (`CharacterMovementComponent.DisableMovement` (`self.CharacterMovement`))
  (`self.FlipCharacter`)
  (`self.GetWorldDecals`))

(event `MC_SetStencil`
  (params (CharacterMeshArray :type "Array of PrimitiveComponent Object Reference") (Stencil :type Integer))
  ;[1 1 1] SetStencil color logic
  (for _array_element CharacterMeshArray
    (`PrimitiveComponent.SetCustomDepthStencilValue` _array_element Stencil)))

(event `PlayLockAnimation`
  ;[1 1 1] LockAnimation logic
  (`self.LockAnimation`))

(event `LockCharacter`
  (params (WorldButton :type "/Game/Core/Widgets/MainMenu/W_WorldButton Object Reference"))
  ;[1 1 1] LockAnimation logic
  (`self.SR_Lock` WorldButton))

(event `SR_Lock`
  (params (WorldButton :type "/Game/Core/Widgets/MainMenu/W_WorldButton Object Reference"))
  ;[1 1 1] LockAnimation logic
  (`self.MC_Lock` WorldButton))

(event `MC_Lock`
  (params (WorldButton :type "/Game/Core/Widgets/MainMenu/W_WorldButton Object Reference"))
  ;[1 1 1] LockAnimation logic
  (if (`self.bCanLock?`)
    (`/Engine/EditorBlueprintResources/StandardMacros.DoOnce` false :!label _label
      (:`Completed`
        (`/Engine/EditorBlueprintResources/StandardMacros.FlipFlop`
          (:`A`
            (set `self.bIsLocked?` true)
            (`/Game/Core/Widgets/MainMenu/W_WorldButton.UpdateTextColor` :`self` WorldButton)
            (`self.LockAnimation`)
            (goto _label :!via `Reset`))
          (:`B`
            (set `self.bIsLocked?` false)
            (`/Game/Core/Widgets/MainMenu/W_WorldButton.UpdateTextColor` WorldButton (struct :`R` 1.0 :`G` 1.0 :`B` 1.0 :`A` 1.0))
            (goto _label :!via `Reset`)))))))

(event `SR_SetStencil`
  (params (CharacterMeshArray :type "Array of PrimitiveComponent Object Reference (by ref)") (Stencil :type Integer))
  ;[1 0 0] new
  (`self.MC_SetStencil` CharacterMeshArray Stencil))

(event `SR_FlipAnim`
  (params (Condition :type Boolean))
  ;[1 1 1] Flip on character switch
  (`self.MC_FlipAnim` Condition))

(event `FlipAnimation`
  (params (NextOrPrevious :type Boolean))
  ;[1 1 1] Flip on character switch
  (if (`self.IsPlayer0?`)
    (`self.SR_FlipAnim` NextOrPrevious)
    (else
      (`self.MC_FlipAnim` NextOrPrevious))))

(event `MC_FlipAnim`
  (params (Condition :type Boolean))
  ;[1 1 1] Flip on character switch
  (`GameplayStatics.PlaySound2D` "/Game/Assets/SFX/MS_ChooseChar.MS_ChooseChar" 1.0 1.0 0.0 null null)
  (if Condition
    (bind (_direction _rotate) (`Timeline|Flip` :!via `PlayFromStart` :!label _label_2)
      (:`Update`
        (`SceneComponent.K2_SetRelativeRotation` (`self.Mesh`) (`KismetMathLibrary.MakeRotator` 0.0 0.0 _rotate) false false)))
    (else
      (goto _label_2 :!via `ReverseFromEnd`))))

(event `FaceOffAnimation`
  (bind _mesh (`self.Mesh`))
  ;[1 1 1] FaceOff animation
  (switch `/Game/Core/Data/Enums/E_CharacterClasses` (`self.eCurrentCharacter`)
    (:`NewEnumerator0`
      (`|PlayMontage` _mesh "/Game/Assets/TikiCharacter/Animations/Spearman/AM_SpearmanLook.AM_SpearmanLook"
        (:`OnCompleted`
          _)))
    (:`NewEnumerator1`
      (`|PlayMontage` _mesh "/Game/Assets/TikiCharacter/Animations/Bonkerman/AM_BonkermanLook.AM_BonkermanLook"
        (:`OnCompleted`
          _)))
    (:`NewEnumerator2`
      (`|PlayMontage` _mesh "/Game/Assets/TikiCharacter/Animations/Magicman/AM_MagicmanLook.AM_MagicmanLook"
        (:`OnCompleted`
          _))))
  (`self.ShowLoadingScreen`))

(fn `FlipCharacter`
  (bind _mesh (`self.Mesh`))
  (if (`self.ActorHasTag` "1")
    (`SceneComponent.SetRelativeScale3D` _mesh (-1.0 1.0 1.0))
    (`MeshComponent.SetOverlayMaterial` _mesh "/Game/Assets/TikiCharacter/Materials/MI_BluePlayer.MI_BluePlayer")
    (else
      (`MeshComponent.SetOverlayMaterial` _mesh "/Game/Assets/TikiCharacter/Materials/MI_RedPlayer.MI_RedPlayer"))))

(fn `GetWorldDecals`
  (bind _outactors (`GameplayStatics.GetAllActorsOfClass` "/Game/Core/Widgets/MainMenu/W_WorldButton.W_WorldButton_C"))
  (for (_array_element _array_index) _outactors
    (switch `int` _array_index
      (:`0`
        (set `self.P1CharacterClassTitle` _array_element))
      (:`1`
        (set `self.P2CharacterClassTitle` _array_element)))))

(fn `OnRep_bCanLock?`
  (bind _asbpc_character_selection (cast `/Game/Core/Blueprints/Input/Controllers/BPC_CharacterSelection` (`GameplayStatics.GetPlayerController` 0)))
  (set `/Game/Core/Blueprints/Input/Controllers/BPC_CharacterSelection.bCanLock?` (`self.bCanLock?`) _asbpc_character_selection))

(fn `OnRep_CurrentTextCharacter`
  (bind _p1characterclasstitle (`self.P1CharacterClassTitle`))
  (bind _p2characterclasstitle (`self.P2CharacterClassTitle`))
  (bind _currenttextcharacter (`self.CurrentTextCharacter`))
  (if (`self.ActorHasTag` self "0")
    (`/Engine/EditorBlueprintResources/StandardMacros.IsValid` _p1characterclasstitle
      (:`Is Valid`
        (`/Game/Core/Widgets/MainMenu/W_WorldButton.UpdateImage` _p1characterclasstitle _currenttextcharacter)))
    (else
      (`/Engine/EditorBlueprintResources/StandardMacros.IsValid` _p2characterclasstitle
        (:`Is Valid`
          (`/Game/Core/Widgets/MainMenu/W_WorldButton.UpdateImage` _p2characterclasstitle _currenttextcharacter))))))

(fn `OnRep_eCurrentCharacter`
  (bind _mesh (`self.Mesh`))
  (switch `/Game/Core/Data/Enums/E_CharacterClasses` (`self.eCurrentCharacter`)
    (:`NewEnumerator0`
      (`SkeletalMeshComponent.SetAnimInstanceClass` _mesh "/Game/Assets/TikiCharacter/Animations/Spearman/ABP_Spearman.ABP_Spearman_C")
      (`self.SetSpearman`)
      (set `self.CurrentTextCharacter` "/Game/Assets/UI/Images/MenuButtons/SPEARMAN.SPEARMAN"))
    (:`NewEnumerator1`
      (`SkeletalMeshComponent.SetAnimInstanceClass` _mesh "/Game/Assets/TikiCharacter/Animations/Bonkerman/ABP_Bonkerman.ABP_Bonkerman_C")
      (`self.SetBonkerman`)
      (set `self.CurrentTextCharacter` "/Game/Assets/UI/Images/MenuButtons/BONKERMAN.BONKERMAN"))
    (:`NewEnumerator2`
      (`SkeletalMeshComponent.SetAnimInstanceClass` _mesh "/Game/Assets/TikiCharacter/Animations/Magicman/ABP_Magicman.ABP_Magicman_C")
      (`self.SetMagicman`)
      (set `self.CurrentTextCharacter` "/Game/Assets/UI/Images/MenuButtons/MAGICMAN.MAGICMAN"))))

(fn `SetBonkerman`
  (bind _bonkermanmesh (`self.BonkermanMesh`))
  (for _array_element (`self.AllSkeletalMeshes`)
    (`SkinnedMeshComponent.SetLeaderPoseComponent` _array_element (`self.Mesh`) false false))
  (`|ExecutionSequence`
    (:`then_0`
      (set `self.ArmDecor2Visability` true))
    (:`then_1`
      (set `self.Eye1Visability` false))
    (:`then_2`
      (set `self.Horn1Visability` false))
    (:`then_3`
      (set `self.HornVisability` true))
    (:`then_4`
      (set `self.ArmDecor1Visability` false))
    (:`then_5`
      (set `self.Eye2Visability` true))
    (:`then_6`
      (set `self.Eye3Visability` false))
    (:`then_7`
      (set `self.HeadDecorVisability` false))
    (:`then_8`
      (set `self.MaskDecorVisability` false))
    (:`then_9`
      (set `self.MaskDecorBoneVisability` false))
    (:`then_10`
      (set `self.Mouth1Visability` false))
    (:`then_11`
      (set `self.Mouth2Visability` true))
    (:`then_12`
      (set `self.Mouth3Visability` false))
    (:`then_13`
      (set `self.TailVisability` true))
    (:`then_14`
      (set `self.ScullVisability` false))
    (:`then_15`
      (set `self.StaffVisability` false))
    (:`then_16`
      (set `self.SpearVisability` false))
    (:`then_17`
      (set `self.BatVisability` true))
    (:`then_18`
      (if (`self.Bonkerman Unlocked`)
        (set `self.bCanLock?` true)
        (`self.SetStencil` _bonkermanmesh)
        (else
          (set `self.bCanLock?` false)
          (`self.SetStencil` _bonkermanmesh 1))))))

(fn `SetMagicman`
  (bind _magicmanmesh (`self.MagicmanMesh`))
  (for _array_element (`self.AllSkeletalMeshes`)
    (`SkinnedMeshComponent.SetLeaderPoseComponent` _array_element (`self.Mesh`) false false))
  (`|ExecutionSequence`
    (:`then_0`
      (set `self.ArmDecor2Visability` false))
    (:`then_1`
      (set `self.Eye1Visability` false))
    (:`then_2`
      (set `self.Horn1Visability` false))
    (:`then_3`
      (set `self.HornVisability` false))
    (:`then_4`
      (set `self.ArmDecor1Visability` true))
    (:`then_5`
      (set `self.Eye2Visability` true))
    (:`then_6`
      (set `self.Eye3Visability` false))
    (:`then_7`
      (set `self.HeadDecorVisability` false))
    (:`then_8`
      (set `self.MaskDecorVisability` false))
    (:`then_9`
      (set `self.MaskDecorBoneVisability` true))
    (:`then_10`
      (set `self.Mouth1Visability` false))
    (:`then_11`
      (set `self.Mouth2Visability` true))
    (:`then_12`
      (set `self.Mouth3Visability` false))
    (:`then_13`
      (set `self.TailVisability` true))
    (:`then_14`
      (set `self.ScullVisability` false))
    (:`then_15`
      (set `self.StaffVisability` true))
    (:`then_16`
      (set `self.SpearVisability` false))
    (:`then_17`
      (set `self.BatVisability` false))
    (:`then_18`
      (if (`self.Magicman Unlocked`)
        (set `self.bCanLock?` true)
        (`self.SetStencil` _magicmanmesh)
        (else
          (set `self.bCanLock?` false)
          (`self.SetStencil` _magicmanmesh 1))))))

(fn `SetSpearman`
  (for _array_element (`self.AllSkeletalMeshes`)
    (`SkinnedMeshComponent.SetLeaderPoseComponent` _array_element (`self.Mesh`) false false))
  (`|ExecutionSequence`
    (:`then_0`
      (set `self.ArmDecor2Visability` false))
    (:`then_1`
      (set `self.Eye1Visability` false))
    (:`then_2`
      (set `self.Horn1Visability` false))
    (:`then_3`
      (set `self.HornVisability` false))
    (:`then_4`
      (set `self.ArmDecor1Visability` false))
    (:`then_5`
      (set `self.Eye2Visability` true))
    (:`then_6`
      (set `self.Eye3Visability` false))
    (:`then_7`
      (set `self.HeadDecorVisability` false))
    (:`then_8`
      (set `self.MaskDecorVisability` true))
    (:`then_9`
      (set `self.MaskDecorBoneVisability` false))
    (:`then_10`
      (set `self.Mouth1Visability` false))
    (:`then_11`
      (set `self.Mouth2Visability` true))
    (:`then_12`
      (set `self.Mouth3Visability` false))
    (:`then_13`
      (set `self.TailVisability` false))
    (:`then_14`
      (set `self.ScullVisability` false))
    (:`then_15`
      (set `self.StaffVisability` false))
    (:`then_16`
      (set `self.SpearVisability` true))
    (:`then_17`
      (set `self.BatVisability` false))
    (:`then_18`
      (set `self.bCanLock?` true)
      (`self.SetStencil` (`self.SpearmanMesh`)))))

(fn `UserConstructionScript`
  (`parent.UserConstructionScript`)
  (set `self.eCurrentCharacter` "NewEnumerator0"))