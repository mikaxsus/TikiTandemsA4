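; BP_EndScreen is a replicated end-screen character that shows winner or loser animations for the Spearman, Bonkerman or Magicman class.
; Team setup functions derive the character from class-name substrings and pick an overlay material by arena type and team, applied through RepNotify.
; A server-to-multicast event plays delayed montages chosen by the "Winner" tag, while looping timers trigger randomly delayed follow-up lock or cry montages.
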(event `self.ReceiveBeginPlay`
  ;[1 1 1] Animation logic
  (`parent.ReceiveBeginPlay`))

(event `SR_PlayAnimations`
  (params (Class :type "Object Class Reference"))
  ;[1 1 1] Animation logic
  (`self.MC_PlayAnimations` Class))

(event `LoopSpearman`
  ;[1 1 1] Animation logic
  (`self.PlayAnimations` false "/Game/Assets/TikiCharacter/Animations/Spearman/AM_LockSpearman.AM_LockSpearman" "/Game/Assets/TikiCharacter/Animations/Shared/AM_Cry.AM_Cry"))

(event `MC_PlayAnimations`
  (params (Class :type "Object Class Reference"))
  ;[1 1 1] Animation logic
  (`self.SwitchOnBP_TikiClass` Class)
  (switch `/Game/Core/Data/Enums/E_CharacterClasses` (`self.eCurrentCharacter`)
    (:`NewEnumerator0`
      (`self.PlayAnimations` true "/Game/Assets/TikiCharacter/Animations/Spearman/AM_LockSpearman.AM_LockSpearman" "/Game/Assets/TikiCharacter/Animations/Shared/AM_LoseAnim.AM_LoseAnim")
      (`KismetSystemLibrary.K2_SetTimerDelegate` (delegate `LoopSpearman`) 5.0 true))
    (:`NewEnumerator1`
      (`self.PlayAnimations` true "/Game/Assets/TikiCharacter/Animations/Bonkerman/AM_BonkermanWin.AM_BonkermanWin" "/Game/Assets/TikiCharacter/Animations/Shared/AM_LoseAnim.AM_LoseAnim")
      (`KismetSystemLibrary.K2_SetTimerDelegate` (delegate `LoopBonkerman`) 5.0 true))
    (:`NewEnumerator2`
      (`self.PlayAnimations` true "/Game/Assets/TikiCharacter/Animations/Magicman/AM_Magicman_Win.AM_Magicman_Win" "/Game/Assets/TikiCharacter/Animations/Shared/AM_LoseAnim.AM_LoseAnim")
      (`KismetSystemLibrary.K2_SetTimerDelegate` (delegate `LoopMagicman`) 5.0 true))))

(event `LoopBonkerman`
  ;[1 1 1] Animation logic
  (`self.PlayAnimations` false "/Game/Assets/TikiCharacter/Animations/Bonkerman/AM_LockBonkerman.AM_LockBonkerman" "/Game/Assets/TikiCharacter/Animations/Shared/AM_Cry.AM_Cry"))

(event `LoopMagicman`
  ;[1 1 1] Animation logic
  (`self.PlayAnimations` false "/Game/Assets/TikiCharacter/Animations/Magicman/AM_LockMagicMan.AM_LockMagicMan" "/Game/Assets/TikiCharacter/Animations/Shared/AM_Cry.AM_Cry"))

(fn `OnRep_aSadAnimation`
  (`SkeletalMeshComponent.SetAnimInstanceClass` (`self.Mesh`) (`self.aSadAnimation`)))

(fn `OnRep_mOverlayMaterial`
  (`MeshComponent.SetOverlayMaterial` (`self.Mesh`) (`self.mOverlayMaterial`)))

(fn `SetLoserTeam`
  (params (Class :type "Object Class Reference") (ArenaType :type "/Game/Core/Data/Enums/E_ArenaType Enum" :default "NewEnumerator0") (WhichTeam :type "/Game/Core/Data/Enums/E_Team Enum" :default "NewEnumerator0"))
  (`self.SwitchOnBP_TikiClass` Class)
  (`self.SetTeamColor` ArenaType WhichTeam))

(fn `SetTeamColor`
  (params (ArenaType :type "/Game/Core/Data/Enums/E_ArenaType Enum" :default "NewEnumerator0") (WhichTeam :type "/Game/Core/Data/Enums/E_Team Enum" :default "NewEnumerator0"))
  (switch `/Game/Core/Data/Enums/E_ArenaType` ArenaType
    (:`NewEnumerator0`
      (switch `/Game/Core/Data/Enums/E_Team` WhichTeam
        (:`NewEnumerator0`
          (set `self.mOverlayMaterial` "/Game/Assets/TikiCharacter/Materials/MI_RedPlayer.MI_RedPlayer"))
        (:`NewEnumerator1`
          (set `self.mOverlayMaterial` "/Game/Assets/TikiCharacter/Materials/MI_BluePlayer.MI_BluePlayer"))))
    (:`NewEnumerator1`
      (switch `/Game/Core/Data/Enums/E_Team` WhichTeam
        (:`NewEnumerator0`
          (set `self.mOverlayMaterial` "/Game/Assets/TikiCharacter/Materials/MI_PurplePLayer.MI_PurplePLayer"))
        (:`NewEnumerator1`
          (set `self.mOverlayMaterial` "/Game/Assets/TikiCharacter/Materials/MI_YellowPlayer.MI_YellowPlayer"))))))

(fn `SetWinnerTeam`
  (params (Class :type "Object Class Reference") (ArenaType :type "/Game/Core/Data/Enums/E_ArenaType Enum" :default "NewEnumerator0") (WhichTeam :type "/Game/Core/Data/Enums/E_Team Enum" :default "NewEnumerator0"))
  (`self.SwitchOnBP_TikiClass` Class)
  (`self.SetTeamColor` ArenaType WhichTeam))

(fn `UserConstructionScript`
  (`parent.UserConstructionScript`))