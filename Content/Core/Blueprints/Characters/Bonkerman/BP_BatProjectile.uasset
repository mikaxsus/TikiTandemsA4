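; Bat projectile for Bonkerman that, on overlap, deals clamped launch damage to BP_Tiki players or damages BP_WinCon totems, recording the struck part and location.
; A player hit also stops projectile movement, turns the bat into a physics body with an applied force, and plays a sound and impact effect.
; SetVFX picks a player or totem dust effect, passed through server and multicast events.
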(event `SR_VFX`
  (params (SystemTemplate :type "NiagaraSystem Object Reference") (Location :type "Vector Structure"))
  (`self.MC_VFX` SystemTemplate Location))

(event `self.Collision.OnComponentBeginOverlap`
  (params (OverlappedComponent :type "PrimitiveComponent Object Reference") (OtherActor :type "Actor Object Reference") (OtherComp :type "PrimitiveComponent Object Reference") (OtherBodyIndex :type Integer) (bFromSweep :type Boolean) (SweepResult :type "HitResult Structure (by ref)"))
  (bind _returnvalue (`self.K2_GetActorLocation`))
  (bind _flaunchstrength (`self.fLaunchStrength`))
  (bind _vfxtype (`self.VFXType`))
  (if (== OtherActor (`self.Instigator`))
    (cast `/Game/Core/Blueprints/TikiCharacter/Blueprint/BP_Tiki` OtherActor
      (:`then`
        (`self.IfPlayerHit` OtherActor _flaunchstrength)
        (`self.SetVFX` :!label _label)
        (`self.IfHit`)
        (`GameplayStatics.PlaySoundAtLocation` "/Game/Assets/SFX/MS_FootSteps.MS_FootSteps" (`self.K2_GetActorLocation`) (struct) 1.0 1.0 0.0 null null null null)
        (if (`KismetSystemLibrary.IsServer`)
          (`self.SR_VFX` _vfxtype _returnvalue)
          (else
            (`self.MC_VFX` _vfxtype _returnvalue))))
      (:`CastFailed`
        (`self.IfTotemHit` OtherActor OtherComp _flaunchstrength)
        (goto _label :!via `Totem`)))))

(event `MC_VFX`
  (params (SystemTemplate :type "NiagaraSystem Object Reference") (Location :type "Vector Structure"))
  (`NiagaraFunctionLibrary.SpawnSystemAtLocation` SystemTemplate Location))

(event `SR_SetVFX`
  (params (VFXType :type "NiagaraSystem Object Reference"))
  (`self.MC_SetVFX` VFXType))

(event `MC_SetVFX`
  (params (VFXType :type "NiagaraSystem Object Reference"))
  (set `self.VFXType` VFXType))

(fn `IfHit`
  (bind _bat (`self.Bat`))
  (`PrimitiveComponent.SetCollisionEnabled` (`self.Collision`) "PhysicsOnly")
  (`ActorComponent.Deactivate` (`self.ProjectileMovement`))
  (`PrimitiveComponent.SetSimulatePhysics` _bat true)
  (`PrimitiveComponent.SetCollisionEnabled` _bat "PhysicsOnly")
  (`PrimitiveComponent.AddForce` _bat (`self.Maths`) "None" false))

(fn `IfPlayerHit`
  (params (Object :type "Object Object Reference") (Value :type "Float (double-precision)"))
  (bind _asbp_tiki (cast `/Game/Core/Blueprints/TikiCharacter/Blueprint/BP_Tiki` Object))
  (`GameplayStatics.ApplyDamage` _asbp_tiki (`KismetMathLibrary.FClamp` Value 0.3) null self "/Game/Core/Data/DamageTypes/DT_Launch.DT_Launch_C"))

(fn `IfTotemHit`
  (params (Object :type "Object Object Reference") (TotemPartHit :type "PrimitiveComponent Object Reference") (BaseDamage :type "Float (single-precision)"))
  (bind _asbp_win_con (cast `/Game/Core/Blueprints/WinCondition/BP_WinCon` Object))
  (set `/Game/Core/Blueprints/WinCondition/BP_WinCon.HitTotemPart` TotemPartHit _asbp_win_con)
  (set `/Game/Core/Blueprints/WinCondition/BP_WinCon.vHitLocation` (- (`self.K2_GetActorLocation`) (20.0 0.0 0.0)) _asbp_win_con)
  (`GameplayStatics.ApplyDamage` _asbp_win_con BaseDamage null (`self.Instigator`)))

(fn `UserConstructionScript`)