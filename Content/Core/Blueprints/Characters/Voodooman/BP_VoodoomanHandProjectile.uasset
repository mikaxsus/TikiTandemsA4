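; Voodooman's hand projectile, which rises from a circle, homes in on the nearest non-instigator Tiki and grabs it with stun damage.
; Montage and timelines drive the rise and wobble, then a delayed search sets the homing target.
; A Tiki overlap stops movement and plays the grab, then server/multicast VFX events show the impact and destroy the actor.
; The construction script attaches Niagara effects to hand sockets.
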(event `self.ReceiveBeginPlay`
  (bind _returnvalue (`self.K2_GetActorLocation`))
  (`|PlayMontage` (`self.Hand`) "/Game/Assets/TikiCharacter/Animations/Voodooman/A_HandSpawn_Montage.A_HandSpawn_Montage"
    (:`then`
      (bind (_direction _zaxis) (`Timeline|Rise` :!via `PlayFromStart`)
        (:`Update`
          (`SceneComponent.K2_SetRelativeLocation` (`self.Hand`) (`KismetMathLibrary.MakeVector` 0.0 0.0 _zaxis) false false))
        (:`Finished`
          (`KismetSystemLibrary.Delay` 0.1)
          (if (`KismetSystemLibrary.IsServer`)
            (`self.SR_VFX` "/Niagara/DefaultAssets/Templates/Systems/RadialBurst.RadialBurst" _returnvalue)
            (else
              (`self.MC_VFX` "/Niagara/DefaultAssets/Templates/Systems/RadialBurst.RadialBurst" _returnvalue)))
          (`KismetSystemLibrary.Delay` 0.05)
          (`ActorComponent.K2_DestroyComponent` (`self.Circle`)))))
    (:`OnCompleted`
      (`|ExecutionSequence`
        (:`then_0`
          (bind (_direction_2 _zaxis_2) (`Timeline|Wobble` :!via `PlayFromStart`)
            (:`Update`
              (`SceneComponent.K2_SetRelativeLocation` (`self.Hand`) (`KismetMathLibrary.MakeVector` 0.0 0.0 _zaxis_2) false false))))
        (:`then_1`
          (`KismetSystemLibrary.Delay` 1.5)
          (`self.FindHomingTarget`))))))

(event `self.Collision.OnComponentBeginOverlap`
  (params (OverlappedComponent :type "PrimitiveComponent Object Reference") (OtherActor :type "Actor Object Reference") (OtherComp :type "PrimitiveComponent Object Reference") (OtherBodyIndex :type Integer) (bFromSweep :type Boolean) (SweepResult :type "HitResult Structure (by ref)"))
  (bind _returnvalue (+ (`self.K2_GetActorLocation`) (0.0 0.0 50.0)))
  (if (!= OtherActor (`self.Instigator`))
    (bind _asbp_tiki (cast `/Game/Core/Blueprints/TikiCharacter/Blueprint/BP_Tiki` OtherActor))
    (`self.IfHitPlayer` _asbp_tiki)
    (`MovementComponent.StopMovementImmediately` (`self.ProjectileMovement`))
    (`|PlayMontage` (`self.Hand`) "/Game/Assets/TikiCharacter/Animations/Voodooman/A_HandGrab_Montage.A_HandGrab_Montage" 2.0
      (:`OnBlendOut`
        (if (`KismetSystemLibrary.IsServer`)
          (`self.SR_VFX` "/Game/Assets/VFX/Flipbook_VFX/Shared/Particles/Lightning/NS_ShootChakram.NS_ShootChakram" _returnvalue true)
          (else
            (`self.MC_VFX` "/Game/Assets/VFX/Flipbook_VFX/Shared/Particles/Lightning/NS_ShootChakram.NS_ShootChakram" _returnvalue true)))))))

(event `SR_VFX`
  (params (SystemTemplate :type "NiagaraSystem Object Reference") (Location :type "Vector Structure") (`FinalHit?` :type Boolean))
  (`self.MC_VFX` SystemTemplate Location `FinalHit?`))

(event `MC_VFX`
  (params (SystemTemplate :type "NiagaraSystem Object Reference") (Location :type "Vector Structure") (`FinalHit?` :type Boolean))
  (bind _returnvalue (`NiagaraFunctionLibrary.SpawnSystemAtLocation` SystemTemplate Location))
  (if `FinalHit?`
    (`NiagaraComponent.SetVariableFloat` _returnvalue "SpriteSize" 650.0)
    (`GameplayStatics.PlaySoundAtLocation` "/Game/Assets/SFX/MS_MagicImpact.MS_MagicImpact" (`self.K2_GetActorLocation`) (struct) 1.0 1.0 0.0 null null null null)
    (`self.K2_DestroyActor`)))

(fn `CreateVFX`
  (locals (VFX :type "NiagaraComponent Object Reference"))
  (bind _vfx (`local.VFX`))
  (bind _hand (`self.Hand`))
  (for _array_element (`SceneComponent.GetAllSocketNames` _hand)
    (bind _returnvalue (`KismetStringLibrary.Conv_NameToString` _array_element))
    (if (`KismetStringLibrary.Contains` _returnvalue "socket")
      (bind _returnvalue_2 (`AddComponent|NODE_AddNiagaraComponent-1`))
      (set `local.VFX` _returnvalue_2)
      (if (`KismetStringLibrary.Contains` _returnvalue "00_socket")
        (`NiagaraComponent.SetVariableFloat` _vfx "Width" 200.0)
        (else
          (`NiagaraComponent.SetVariableFloat` _vfx "Width" 60.0)))
      (`SceneComponent.K2_AttachToComponent` _vfx _hand _array_element "SnapToTarget" "SnapToTarget" "SnapToTarget" true))))

(fn `FindHomingTarget`
  (locals (iNearestIndex :type Integer))
  (set `self.fClosestDistance` 2000000000.0)
  (bind _outactors (`GameplayStatics.GetAllActorsOfClass` "/Game/Core/Blueprints/TikiCharacter/Blueprint/BP_Tiki.BP_Tiki_C"))
  (for (_array_element _array_index) _outactors
    (if (!= _array_element (`self.Instigator`))
      (bind _returnvalue (`KismetMathLibrary.Vector_Distance` (`self.K2_GetActorLocation` _array_element) (`SceneComponent.K2_GetComponentLocation` (`self.DefaultSceneRoot`))))
      (if (< _returnvalue (`self.fClosestDistance`))
        (set `local.iNearestIndex` _array_index)
        (set `self.fClosestDistance` _returnvalue))))
  (set `ProjectileMovementComponent.HomingTargetComponent` (`Actor.RootComponent` (`|GetArrayItem` _outactors (`local.iNearestIndex`))) (`self.ProjectileMovement`)))

(fn `IfHitPlayer`
  (params (Object :type "Object Object Reference"))
  (bind _asbp_tiki (cast `/Game/Core/Blueprints/TikiCharacter/Blueprint/BP_Tiki` Object))
  (`GameplayStatics.ApplyDamage` _asbp_tiki (/ (`self.fLaunchStrength`) 1.2) null (`self.Instigator`) "/Game/Core/Data/DamageTypes/DT_Stun.DT_Stun_C")
  (`PrimitiveComponent.SetCollisionEnabled` (`self.Collision`) "NoCollision"))

(fn `UserConstructionScript`
  (`self.CreateVFX`))