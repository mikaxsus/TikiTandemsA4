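; Game mode for the Tiki Tandems end screen, which disables splitscreen and presents the winning and losing teams.
; In non-local games, BeginPlay configures each BP_EndScreen actor by its "Winner" tag, using class, team and arena from the game instance, then multicasts animations.
; Swapped-in player controllers are collected, and after a short delay each is told to remove its loading screen.
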(event `self.ReceiveBeginPlay`
  ;[1 1 1] Event BeginPlay
  (`GameplayStatics.SetForceDisableSplitscreen` true)
  (bind _asgi_tiki_tandems (cast `/Game/Core/Blueprints/GameRules/GI_TikiTandems` (`GameplayStatics.GetGameInstance`)))
  (if (not (`/Game/Core/Blueprints/GameRules/GI_TikiTandems.bLocalGame?` _asgi_tiki_tandems))
    (`self.MC_SetPlayers`)))

(event `self.K2_OnSwapPlayerControllers`
  (params (OldPC :type "PlayerController Object Reference") (NewPC :type "PlayerController Object Reference"))
  ;[1 1 1] Event SwapControllers logic
  (`KismetArrayLibrary.Array_Add` (`self.PlayerControllers`) NewPC)
  (`KismetSystemLibrary.Delay` 1.6)
  (for _array_element (`self.PlayerControllers`)
    (bind _asbpc_end_screen (cast `/Game/Core/Blueprints/Input/Controllers/BPC_EndScreen` _array_element))
    (`/Game/Core/Blueprints/Input/Controllers/BPC_EndScreen.CL_RemoveLoadingScreen` _asbpc_end_screen)))

(event `MC_SetPlayers`
  (bind _asgi_tiki_tandems (cast `/Game/Core/Blueprints/GameRules/GI_TikiTandems` (`GameplayStatics.GetGameInstance`) :!pure true))
  (bind (_stloserinfo_characterclass _stloserinfo_playerteam) (break `/Game/Core/Data/CharacterData/ST_EndInfo` (`/Game/Core/Blueprints/GameRules/GI_TikiTandems.stLoserInfo` _asgi_tiki_tandems)))
  (bind (_stwinnerinfo_characterclass _stwinnerinfo_playerteam) (break `/Game/Core/Data/CharacterData/ST_EndInfo` (`/Game/Core/Blueprints/GameRules/GI_TikiTandems.stWinnerInfo` _asgi_tiki_tandems)))
  (bind _earenatype (`/Game/Core/Blueprints/GameRules/GI_TikiTandems.eArenaType` _asgi_tiki_tandems))
  ;[1 1 1] SetPlayers logic
  (bind _outactors (`GameplayStatics.GetAllActorsOfClass` "/Game/Core/Blueprints/Characters/EndScreen/BP_EndScreen.BP_EndScreen_C"))
  (for _array_element _outactors
    (if (`self.ActorHasTag` _array_element "Winner")
      (`/Game/Core/Blueprints/Characters/EndScreen/BP_EndScreen.SetWinnerTeam` _array_element _stwinnerinfo_characterclass _earenatype _stwinnerinfo_playerteam)
      (`/Game/Core/Blueprints/Characters/EndScreen/BP_EndScreen.MC_PlayAnimations` _array_element _stwinnerinfo_characterclass)
      (else
        (set `/Game/Core/Blueprints/Characters/EndScreen/BP_EndScreen.aSadAnimation` "/Game/Assets/TikiCharacter/Animations/Shared/ABP_WildmanLose.ABP_WildmanLose_C" _array_element)
        (`/Game/Core/Blueprints/Characters/EndScreen/BP_EndScreen.SetLoserTeam` _array_element _stloserinfo_characterclass _earenatype _stloserinfo_playerteam)
        (`/Game/Core/Blueprints/Characters/EndScreen/BP_EndScreen.MC_PlayAnimations` _array_element _stloserinfo_characterclass)))))

(fn `UserConstructionScript`)