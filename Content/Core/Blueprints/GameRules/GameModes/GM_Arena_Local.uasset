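; Game mode for local Tiki Tandems arena matches, running setup, intros, match timer and win-screen handoff.
; BeginPlay streams the day or night map, then chains events that recreate players from GameInstance controller and class data and spawn their pawns.
; Per-player intros play sequentially with splitscreen disabled, before cleanup enables controls, team overlays and HUD.
; Tick reads win progress from BP_WinCon rotations; timer expiry quits the game, while EndTheGame stores results.
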(event `self.ReceiveBeginPlay`
  ;[1 1 1] BeginPlay logic
  (`self.SetArenaType`)
  (bind _asgi_tiki_tandems (cast `/Game/Core/Blueprints/GameRules/GI_TikiTandems` (`GameplayStatics.GetGameInstance`)))
  (set `/Game/Core/Blueprints/GameRules/GI_TikiTandems.bLocalGame?` true _asgi_tiki_tandems)
  (`GameplayStatics.SetForceDisableSplitscreen` true)
  (add `self.OnInitialize` (delegate `CreatePlayerControllers`))
  (add `self.OnCreatedPlayerControllers` (delegate `SpawnActors`))
  (add `self.OnSpawnedAllActors` (delegate `StartMatchTiki`))
  (bind _returnvalue (`GameplayStatics.GetActorOfClass` "/Game/Core/Blueprints/WinCondition/BP_WinCon.BP_WinCon_C"))
  (set `self.WinConReference` _returnvalue)
  (bind _outactors (`GameplayStatics.GetAllActorsOfClass` "/Script/Engine.PlayerStart"))
  (set `self.Spawns` _outactors)
  (bind _outactors_2 (`GameplayStatics.GetAllActorsOfClass` "/Script/Engine.PlayerController"))
  (for _array_element _outactors_2
    (`GameplayStatics.RemovePlayer` _array_element true))
  (`self.OnInitialize`))

(event `CreatePlayerControllers`
  ;[1 1 1] BeginPlay logic
  (`self.CreateAllPlayerControllers`))

(event `SpawnActors`
  ;[1 1 1] BeginPlay logic
  (`self.SpawnAllPlayerPawns`))

(event `StartMatchTiki`
  ;[1 1 1] BeginPlay logic
  (`self.HideAllPlayerCharacters`)
  (`self.PlayIntroSequence` 0))

(event `SetArenaType`
  ;[1 1 1] Set arena type logic
  (bind _asgi_tiki_tandems (cast `/Game/Core/Blueprints/GameRules/GI_TikiTandems` (`GameplayStatics.GetGameInstance`)))
  (`GameplayStatics.FlushLevelStreaming`)
  (switch `/Game/Core/Data/Enums/E_ArenaType` (`/Game/Core/Blueprints/GameRules/GI_TikiTandems.eArenaType` _asgi_tiki_tandems)
    (:`NewEnumerator0`
      (`GameplayStatics.LoadStreamLevelBySoftObjectPtr` "/Game/maps/L_DayMap.L_DayMap" true))
    (:`NewEnumerator1`
      (`GameplayStatics.LoadStreamLevelBySoftObjectPtr` "/Game/maps/L_NightMap.L_NightMap" true)
      (bind _outactors (`GameplayStatics.GetAllActorsOfClass` "/Game/Core/Blueprints/Obstacles/BP_Quicksand.BP_Quicksand_C"))
      (for _array_element _outactors
        (message `/Game/Core/Blueprints/Input/Interfaces/BPI_Sync.BIS_QuicksandStart` _array_element)))))

(event `CallHandleStartingNewPlayer`
  (params (NewPlayer :type "PlayerController Object Reference") (iPlayerIndex :type Integer))
  ;[1 1 1] NewPlayer logic
  (`parent.HandleStartingNewPlayer` NewPlayer)
  (bind _asbpc_tiki_arena_local (cast `/Game/Core/Blueprints/Input/Controllers/BPC_TikiArena_Local` NewPlayer))
  (set `/Game/Core/Blueprints/Input/Controllers/BPC_TikiArena_Local.iPlayerIndex` iPlayerIndex _asbpc_tiki_arena_local))

(event `PlayIntroSequence`
  (params (PlayerIndex :type Integer))
  ;[1 1 1] PlayIntroSequences logic
  (bind _asgi_tiki_tandems (cast `/Game/Core/Blueprints/GameRules/GI_TikiTandems` (`GameplayStatics.GetGameInstance`)))
  (bind _asbpc_tiki_arena_local (cast `/Game/Core/Blueprints/Input/Controllers/BPC_TikiArena_Local` (`|GetArrayItem` (`self.PlayerControllers`) PlayerIndex)))
  (`/Game/Core/Blueprints/Input/Controllers/BPC_TikiArena_Local.PlayAnimation` _asbpc_tiki_arena_local (`BlueprintMapLibrary.Map_Find` (`/Game/Core/Blueprints/GameRules/GI_TikiTandems.PlayerClassByID` _asgi_tiki_tandems) PlayerIndex) PlayerIndex)
  (`/Game/Core/Blueprints/Input/Controllers/BPC_TikiArena_Local.CreateSkipButtonWidget` _asbpc_tiki_arena_local)
  (add `MovieSceneSequencePlayer.OnStop` (`/Game/Core/Blueprints/Input/Controllers/BPC_TikiArena_Local.ActivePlayerSequence` _asbpc_tiki_arena_local) (delegate `SequenceEnded`)))

(event `SequenceEnded`
  ;[1 1 1] PlayIntroSequences logic
  (if (!= (stale `PlayIntroSequence` PlayerIndex) (- (`KismetArrayLibrary.Array_Length` (`self.PlayerControllers`)) 1))
    (bind _result (`/Engine/EditorBlueprintResources/StandardMacros.IncrementInt` (stale `PlayIntroSequence` PlayerIndex))
      (:`  `
        (`self.PlayIntroSequence` _result)))
    (else
      (`self.CleanupAndBeginGame`))))

(event `self.ReceiveTick`
  (params (DeltaSeconds :type "Float (single-precision)"))
  (bind _winconreference (`self.WinConReference`))
  (bind (_relativerotation_roll _relativerotation_pitch _relativerotation_yaw) (`KismetMathLibrary.BreakRotator` (`SceneComponent.RelativeRotation` (`/Game/Core/Blueprints/WinCondition/BP_WinCon.WingsBase` _winconreference))))
  (bind (_relativerotation_roll_2 _relativerotation_pitch_2 _relativerotation_yaw_2) (`KismetMathLibrary.BreakRotator` (`SceneComponent.RelativeRotation` (`/Game/Core/Blueprints/WinCondition/BP_WinCon.FistsBase` _winconreference))))
  ;[1 1 1] WinProgress logic
  (set `self.WinProgress` _relativerotation_yaw)
  (set `self.PowerUpProgress` _relativerotation_yaw_2))

(event `StartGameTimer`
  ;[1 1 1] Timer for match logic
  (`KismetSystemLibrary.K2_SetTimerDelegate` (delegate `UpdateGameTimer`) 1.0 true))

(event `UpdateGameTimer`
  ;[1 1 1] Timer for match logic
  (if (== (`self.Seconds`) 0)
    (if (== (`self.Minutes`) 0)
      (`KismetSystemLibrary.QuitGame` null "Quit")
      (else
        (bind _result (`/Engine/EditorBlueprintResources/StandardMacros.DecrementInt` (`self.Minutes`))
          (:`  `
            (set `self.Minutes` _result)
            (set `self.Seconds` 59)))))
    (else
      (bind _result_2 (`/Engine/EditorBlueprintResources/StandardMacros.DecrementInt` (`self.Seconds`))
        (:`  `
          (set `self.Seconds` _result_2))))))

(event `AddControls`
  ;[1 1 1] Add controls and startgame logic
  (for _array_element (`self.PlayerControllers`)
    (bind _asbpc_tiki_arena_local (cast `/Game/Core/Blueprints/Input/Controllers/BPC_TikiArena_Local` _array_element))
    (`/Game/Core/Blueprints/Input/Controllers/BPC_TikiArena_Local.AddInputs` _asbpc_tiki_arena_local)
    (if (== (mod (`/Game/Core/Blueprints/Input/Controllers/BPC_TikiArena_Local.iPlayerIndex` _asbpc_tiki_arena_local) 2) 0)
      (`Controller.SetControlRotation` _asbpc_tiki_arena_local (`KismetMathLibrary.MakeRotator` 0.0 5.0 90.0))
      (else
        (`Controller.SetControlRotation` _asbpc_tiki_arena_local (`KismetMathLibrary.MakeRotator` 0.0 5.0 -90.0))))))

(event `SetTeamOverlay`
  ;[1 1 1] Set team colors/overlay logic
  (for _array_element (`self.PlayerControllers`)
    (bind _asbpc_tiki_arena_local (cast `/Game/Core/Blueprints/Input/Controllers/BPC_TikiArena_Local` _array_element))
    (bind _asbp_tiki (cast `/Game/Core/Blueprints/TikiCharacter/Blueprint/BP_Tiki` (`Controller.K2_GetPawn` _asbpc_tiki_arena_local)))
    (`/Game/Core/Blueprints/TikiCharacter/Blueprint/BP_Tiki.SetTeamOverlayColor` _asbp_tiki (`/Game/Core/Blueprints/Input/Controllers/BPC_TikiArena_Local.iPlayerIndex` _asbpc_tiki_arena_local))))

(event `EndTheGame`
  (params (`WhichTeamWon?` :type "/Game/Core/Data/Enums/E_Team Enum" :default "NewEnumerator0"))
  ;[1 1 1] EndGame logic
  (`WidgetLayoutLibrary.RemoveAllWidgets`)
  (`GameplayStatics.SetGlobalTimeDilation` 0.2)
  (`self.SetWinnerLoser` `WhichTeamWon?`)
  (`KismetSystemLibrary.Delay` 1.5)
  (`GameplayStatics.OpenLevelBySoftObjectPtr` "/Game/maps/L_WinScreen.L_WinScreen"))

(event `CreateArenaWidget`
  ;[1 1 1] Create overlay for totem
  (bind _returnvalue (`|CreateWidget` "/Game/Core/Widgets/NewHUDs/W_GameOverlay_Local.W_GameOverlay_Local_C"))
  (`UserWidget.AddToViewport` _returnvalue 0))

(fn `CleanupAndBeginGame`
  (`GameplayStatics.SetForceDisableSplitscreen` false)
  (bind _outactors (`GameplayStatics.GetAllActorsOfClassWithTag` "/Script/Engine.SkeletalMeshActor" "Cinematic"))
  (for _array_element _outactors
    (`self.K2_DestroyActor` _array_element))
  (bind _outactors_2 (`GameplayStatics.GetAllActorsOfClass` "/Game/Core/Blueprints/TikiCharacter/Blueprint/BP_Tiki.BP_Tiki_C"))
  (for _array_element_2 _outactors_2
    (`self.SetActorHiddenInGame` _array_element_2 false))
  (`self.AddControls`)
  (`self.StartGameTimer`)
  (`self.SetTeamOverlay`)
  (`self.CreateArenaWidget`)
  (return))

(fn `CreateAllPlayerControllers`
  (bind _controllerid (`/Game/Core/Blueprints/GameRules/GI_TikiTandems.ControllerID` (cast `/Game/Core/Blueprints/GameRules/GI_TikiTandems` (`GameplayStatics.GetGameInstance`) :!pure true)))
  (for _index (range (`BlueprintMapLibrary.Map_Length` _controllerid))
    (bind _returnvalue (`GameplayStatics.CreatePlayer` (`BlueprintMapLibrary.Map_Find` _controllerid _index)))
    (`KismetArrayLibrary.Array_Add` (`self.PlayerControllers`) _returnvalue))
  (`self.OnCreatedPlayerControllers`)
  (return))

(fn `HideAllPlayerCharacters`
  (bind _outactors (`GameplayStatics.GetAllActorsOfClass` "/Game/Core/Blueprints/TikiCharacter/Blueprint/BP_Tiki.BP_Tiki_C"))
  (for _array_element _outactors
    (`self.SetActorHiddenInGame` _array_element true))
  (return))

(fn `SetWinnerLoser`
  (params (WinningTeam :type "/Game/Core/Data/Enums/E_Team Enum" :default "NewEnumerator0"))
  (bind _asgi_tiki_tandems (cast `/Game/Core/Blueprints/GameRules/GI_TikiTandems` (`GameplayStatics.GetGameInstance`)))
  (for (_array_element _array_index) (`self.PlayerControllers`)
    (bind _asbpc_tiki_arena_local (cast `/Game/Core/Blueprints/Input/Controllers/BPC_TikiArena_Local` _array_element))
    (bind _eplayerteam (`/Game/Core/Blueprints/Input/Controllers/BPC_TikiArena_Local.ePlayerTeam` _asbpc_tiki_arena_local))
    (if (`|EnumEquality` _eplayerteam WinningTeam)
      (bind _st_endinfo (make `/Game/Core/Data/CharacterData/ST_EndInfo` (`BlueprintMapLibrary.Map_Find` (`/Game/Core/Blueprints/GameRules/GI_TikiTandems.PlayerClassByID` _asgi_tiki_tandems) _array_index) _eplayerteam))
      (set `/Game/Core/Blueprints/GameRules/GI_TikiTandems.stWinnerInfo` _st_endinfo _asgi_tiki_tandems)
      (else
        (set `/Game/Core/Blueprints/GameRules/GI_TikiTandems.stLoserInfo` _st_endinfo _asgi_tiki_tandems)))))

(fn `SpawnAllPlayerPawns`
  (bind _playerclassbyid (`/Game/Core/Blueprints/GameRules/GI_TikiTandems.PlayerClassByID` (cast `/Game/Core/Blueprints/GameRules/GI_TikiTandems` (`GameplayStatics.GetGameInstance`) :!pure true)))
  (for _index (range (`BlueprintMapLibrary.Map_Length` _playerclassbyid))
    (bind _returnvalue (`|SpawnActorFromClass` (`BlueprintMapLibrary.Map_Find` _playerclassbyid _index) (`self.GetTransform` (`|GetArrayItem` (`self.Spawns`) _index)) "Undefined" "MultiplyWithRoot" null null))
    (bind _output (`|GetArrayItem` (`self.PlayerControllers`) _index))
    (`Controller.Possess` _output _returnvalue)
    (`self.CallHandleStartingNewPlayer` _output _index))
  (`self.OnSpawnedAllActors`)
  (return))

(fn `UserConstructionScript`)