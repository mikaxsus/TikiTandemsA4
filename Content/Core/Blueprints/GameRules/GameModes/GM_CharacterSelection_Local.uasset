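; Game mode for the local character selection screen, which sets up two local players on a shared view with splitscreen force-disabled.
; BeginPlay shows a loading screen, then swaps it for the selection widget after a short delay.
; It also creates each player with input disabled, registers the controller with an exit input mapping context, and unlocks Bonkerman and Magicman on every BP_CharacterSelection actor.
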(event `self.ReceiveBeginPlay`
  (`GameplayStatics.SetForceDisableSplitscreen` true)
  (`|ExecutionSequence`
    (:`then_0`
      (`self.ShowLoadingScreen`))
    (:`then_1`
      (for _index (range 2)
        (bind _output_get (set `self.SpawnIndex` _index))
        (`GameplayStatics.CreatePlayer` _output_get)
        (bind _returnvalue (`GameplayStatics.GetPlayerController` _output_get))
        (`self.DisableInput` _returnvalue _returnvalue)
        (`self.CallHandleStartingNewPlayer` _returnvalue)))
    (:`then_2`
      (bind _outactors (`GameplayStatics.GetAllActorsOfClass` "/Game/Core/Blueprints/Characters/CharacterSelector/BP_CharacterSelection.BP_CharacterSelection_C"))
      (for _array_element _outactors
        (set `/Game/Core/Blueprints/Characters/CharacterSelector/BP_CharacterSelection.Bonkerman Unlocked` true _array_element)
        (set `/Game/Core/Blueprints/Characters/CharacterSelector/BP_CharacterSelection.Magicman Unlocked` true _array_element)))))

(event `CallHandleStartingNewPlayer`
  (params (NewPlayer :type "PlayerController Object Reference"))
  (`parent.HandleStartingNewPlayer` NewPlayer)
  (bind _asbpc_character_selection_local (cast `/Game/Core/Blueprints/Input/Controllers/BPC_CharacterSelection_Local` NewPlayer))
  (`/Game/Core/Blueprints/Functions/BFL_General.AddInputMappingContext` _asbpc_character_selection_local "/Game/Core/Blueprints/Input/InputActionMappings/IMC_Exit.IMC_Exit" 1)
  (`KismetArrayLibrary.Array_Add` (`self.PlayerControllers`) NewPlayer))

(event `ShowLoadingScreen`
  ;[1 1 1] Event ShowLoadingScreen logic
  (bind _loadingscreenwidget (`/Game/Core/Blueprints/Functions/BFL_General.CreateLoadingScreen` (`GameplayStatics.GetPlayerController` 0)))
  (set `self.wLoadingScreen` _loadingscreenwidget)
  (`/Engine/EditorBlueprintResources/StandardMacros.DoOnce` false
    (:`Completed`
      (`KismetSystemLibrary.Delay` 1.5)
      (`Widget.RemoveFromParent` (`self.wLoadingScreen`))
      (bind _returnvalue (`|CreateWidget` "/Game/Core/Widgets/CharacterSelection/W_CharacterSelectionScreen.W_CharacterSelectionScreen_C"))
      (bind _output_get (set `self.wCharacterSelection` _returnvalue))
      (`UserWidget.AddToViewport` _output_get 0))))

(fn `UserConstructionScript`)