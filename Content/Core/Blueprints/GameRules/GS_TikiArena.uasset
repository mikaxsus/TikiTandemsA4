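; GS_TikiArena is the Tiki arena game state, running match start, countdown and objective progress.
; CleanupAndBeginGame removes cinematic meshes, unhides Tikis, enables inputs with view direction set by player-index parity, starts the timer and applies team overlays.
; A one-second looping timer counts down and quits the game at zero.
; Tick derives win and power-up progress from the yaw of the BP_WinCon totem's wings and fists.
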(event `MC_StartGameTimer`
  ;[1 1 1] Timer for match logic
  (`KismetSystemLibrary.K2_SetTimerDelegate` (delegate `UpdateGameTimer`) 1.0 true))

(event `UpdateGameTimer`
  ;[1 1 1] Timer for match logic
  (if (== (`self.Seconds`) 0)
    (if (== (`self.Minutes`) 0)
      (`KismetSystemLibrary.QuitGame` null "Quit")
      (else
        (bind _result (`/Engine/EditorBlueprintResources/StandardMacros.DecrementInt` (`self.Minutes`))
          (:`  `
            (set `self.Minutes` _result)
            (set `self.Seconds` 59)))))
    (else
      (bind _result_2 (`/Engine/EditorBlueprintResources/StandardMacros.DecrementInt` (`self.Seconds`))
        (:`  `
          (set `self.Seconds` _result_2))))))

(event `self.ReceiveTick`
  (params (DeltaSeconds :type "Float (single-precision)"))
  (bind _totem (`self.Totem`))
  (bind (_relativerotation_roll _relativerotation_pitch _relativerotation_yaw) (`KismetMathLibrary.BreakRotator` (`SceneComponent.RelativeRotation` (`/Game/Core/Blueprints/WinCondition/BP_WinCon.WingsBase` _totem))))
  (bind (_relativerotation_roll_2 _relativerotation_pitch_2 _relativerotation_yaw_2) (`KismetMathLibrary.BreakRotator` (`SceneComponent.RelativeRotation` (`/Game/Core/Blueprints/WinCondition/BP_WinCon.FistsBase` _totem))))
  ;[1 1 1] WinCon logic
  (set `self.WinProgress` _relativerotation_yaw)
  (set `self.PowerUpProgress` _relativerotation_yaw_2))

(event `self.ReceiveBeginPlay`
  ;[1 1 1] BeginPlay logic
  (bind _returnvalue (`GameplayStatics.GetActorOfClass` "/Game/Core/Blueprints/WinCondition/BP_WinCon.BP_WinCon_C"))
  (set `self.Totem` _returnvalue))

(event `MC_AddControls`
  ;[1 1 1] Add controls and startgame logic
  (for _array_element (`self.PlayerArray`)
    (bind _asbpc_arena (cast `/Game/Core/Blueprints/Input/Controllers/BPC_Arena` (`PlayerState.GetPlayerController` _array_element)))
    (`/Game/Core/Blueprints/Input/Controllers/BPC_Arena.CL_AddInputs` _asbpc_arena)
    (if (== (mod (`/Game/Core/Blueprints/Input/Controllers/BPC_Arena.iPlayerIndex` _asbpc_arena) 2) 0)
      (`Controller.SetControlRotation` _asbpc_arena (`KismetMathLibrary.MakeRotator` 0.0 5.0 90.0))
      (else
        (`Controller.SetControlRotation` _asbpc_arena (`KismetMathLibrary.MakeRotator` 0.0 5.0 -90.0))))))

(event `CL_SetTeamOverlay`
  ;[1 1 1] Set team colors/overlay logic
  (`KismetSystemLibrary.Delay` 0.2)
  (for _array_element (`self.PlayerArray`)
    (bind _asbpc_arena (cast `/Game/Core/Blueprints/Input/Controllers/BPC_Arena` (`PlayerState.GetPlayerController` _array_element)))
    (bind _asbp_tiki (cast `/Game/Core/Blueprints/TikiCharacter/Blueprint/BP_Tiki` (`Controller.K2_GetPawn` _asbpc_arena)))
    (`/Game/Core/Blueprints/TikiCharacter/Blueprint/BP_Tiki.SR_SetTeamOverlayColor` _asbp_tiki (`/Game/Core/Blueprints/Input/Controllers/BPC_Arena.iPlayerIndex` _asbpc_arena))))

(fn `CleanupAndBeginGame`
  (bind _outactors (`GameplayStatics.GetAllActorsOfClassWithTag` "/Script/Engine.SkeletalMeshActor" "Cinematic"))
  (for _array_element _outactors
    (`self.K2_DestroyActor` _array_element))
  (bind _outactors_2 (`GameplayStatics.GetAllActorsOfClass` "/Game/Core/Blueprints/TikiCharacter/Blueprint/BP_Tiki.BP_Tiki_C"))
  (for _array_element_2 _outactors_2
    (`self.SetActorHiddenInGame` _array_element_2 false))
  (`self.MC_AddControls`)
  (`self.MC_StartGameTimer`)
  (`self.CL_SetTeamOverlay`)
  (return))

(fn `SetTotemReferences`
  (bind _returnvalue (`GameplayStatics.GetActorOfClass` "/Game/Core/Blueprints/WinCondition/BP_WinCon.BP_WinCon_C"))
  (set `self.WinConRef` (`/Game/Core/Blueprints/WinCondition/BP_WinCon.WingsBase` _returnvalue))
  (set `self.PowerUpRef` (`/Game/Core/Blueprints/WinCondition/BP_WinCon.FistsBase` _returnvalue)))

(fn `UserConstructionScript`)