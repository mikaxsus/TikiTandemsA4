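; BP_WinCon is the Tiki Tandems win-condition totem, whose wings and fists rotate when damaged, styled for Day or Night arenas.
; Hit distance to front/back markers picks direction, and damage scales timeline-driven turns applied through OnReps.
; Fist yaw sets directional boosts that feed wing rotation, locking the fists near full boost.
; Hits trigger emissive flashes colored by direction and arena, while Tick's wing-yaw check leads only to empty DoOnce nodes.
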(event `self.ReceiveBeginPlay`
  ;[1 1 1] Event BeginPlay
  (bind _asgi_tiki_tandems (cast `/Game/Core/Blueprints/GameRules/GI_TikiTandems` (`GameplayStatics.GetGameInstance`)))
  (set `self.eArena` (`/Game/Core/Blueprints/GameRules/GI_TikiTandems.eArenaType` _asgi_tiki_tandems))
  (`self.SetTotemStyle`))

(event `self.ReceiveAnyDamage`
  (params (Damage :type "Float (single-precision)") (DamageType :type "DamageType Object Reference") (InstigatedBy :type "Controller Object Reference") (DamageCauser :type "Actor Object Reference"))
  ;[1 1 1] EventAnyDamage
  (if (`self.bCanBeDamaged`)
    (`self.WhichTotemPart`)
    (`self.TotemRotation`)
    (`self.StopTotemRotation`)
    (`self.RotateTotem` (`self.eTotemRotation`) Damage (`self.eTotemHitPart`))
    (`KismetSystemLibrary.Delay` 0.08)
    (`/Engine/EditorBlueprintResources/ActorMacros.Switch Has Authority`
      (:`Authority`
        (`self.SR_LightUpTotem`))
      (:`Remote`
        (`self.MC_LightUpTotem`)))))

(event `StopTurningWings`
  ;[1 1 1] StopTurningLogic
  (`self.StopWingsClockwise`)
  (`self.StopWingsCounterClockwise`)
  (set `self.fCurrentWingsRotation` (`self.CurrentWingsRotation`)))

(event `self.ReceiveTick`
  (params (DeltaSeconds :type "Float (single-precision)"))
  (bind (_returnvalue_roll _returnvalue_pitch _returnvalue_yaw) (`KismetMathLibrary.BreakRotator` (`SceneComponent.K2_GetComponentRotation` (`self.WingsBase`))))
  ;[1 1 1] EventTick
  (`|ExecutionSequence`
    (:`then_0`
      (if (not (`self.bAreFistsLocked?`))
        (`self.FistsPowerUp`)))
    (:`then_1`
      (if (>= _returnvalue_yaw 170.0)
        (`/Engine/EditorBlueprintResources/StandardMacros.DoOnce` false)
        (elif (>= _returnvalue_yaw -170.0)
          (`/Engine/EditorBlueprintResources/StandardMacros.DoOnce` false))))))

(event `StopTurningFists`
  ;[1 1 1] StopTurningLogic
  (`self.StopFistsClockwise`)
  (`self.StopFistsCounterClockwise`)
  (set `self.fCurrentFistsRotation` (`self.CurrentFistsRotation`)))

(event `MC_LightUpTotem`
  ;[1 1 1] TotemEmissiveLogic
  (`self.ResetEmissive`)
  (bind (_direction _emissive) (`Timeline|LightUp` :!via `PlayFromStart`)
    (:`Update`
      (set `self.fEmissive` _emissive))))

(event `SR_LightUpTotem`
  ;[1 1 1] TotemEmissiveLogic
  (`self.MC_LightUpTotem`))

(event `StopWingsClockwise`
  ;[1 1 1] TotemRotationLogic
  (`|ExecutionSequence`
    (:`then_0`
      (set `self.fCurrentWingsRotation` (`self.CurrentWingsRotation`) :!label _label))
    (:`then_1`
      (bind (_direction _wingclockwiserotation) (`Timeline|WingsClockwiseRotation` :!via `Stop` :!label _label_2)
        (:`Update`
          (set `self.fWingRotation` _wingclockwiserotation))
        (:`Finished`
          (goto _label))))))

(event `RotateTotem`
  (params (Rotation :type "/Game/Core/Data/Enums/E_TotemRotation Enum" :default "NewEnumerator0") (TurnAmount :type "Float (double-precision)") (TotemPartHit :type "/Game/Core/Data/Enums/E_TotemPart Enum" :default "NewEnumerator0"))
  ;[1 1 1] TotemRotationLogic
  (set `self.fTurnAmount` TurnAmount)
  (switch `/Game/Core/Data/Enums/E_TotemRotation` Rotation
    (:`NewEnumerator0`
      (switch `/Game/Core/Data/Enums/E_TotemPart` TotemPartHit
        (:`NewEnumerator0`
          (set `self.bAreWingsTurning?` true :!label _label_3)
          (goto _label_2 :!via `PlayFromStart`))
        (:`NewEnumerator1`
          (goto _label_3))
        (:`NewEnumerator2`
          _)
        (:`NewEnumerator3`
          _))
      (if (not (`self.bAreFistsLocked?`))
        (set `self.bAreFistsTurning?` true)
        (bind (_direction _fistsclockwiserotation) (`Timeline|FistsClockwiseRotation` :!via `PlayFromStart` :!label _label_4)
          (:`Update`
            (set `self.fFistRotation` _fistsclockwiserotation))
          (:`Finished`
            (set `self.fCurrentFistsRotation` (`self.CurrentFistsRotation`) :!label _label_5)))))
    (:`NewEnumerator1`
      (switch `/Game/Core/Data/Enums/E_TotemPart` TotemPartHit
        (:`NewEnumerator0`
          (set `self.bAreWingsTurning?` true :!label _label_6)
          (bind (_direction_2 _wingcounterclockwiserotation) (`Timeline|WingsCounterClockwiseRotation` :!via `PlayFromStart` :!label _label_7)
            (:`Update`
              (set `self.fWingRotation` _wingcounterclockwiserotation))
            (:`Finished`
              (set `self.fCurrentWingsRotation` (`self.CurrentWingsRotation`) :!label _label_8))))
        (:`NewEnumerator1`
          (goto _label_6))
        (:`NewEnumerator2`
          (if (not (`self.bAreFistsLocked?`)) :!label _label_9
            (set `self.bAreFistsTurning?` true)
            (bind (_direction_3 _fistscounterclockwiserotation) (`Timeline|FistsCounterClockwiseRotation` :!via `PlayFromStart` :!label _label_10)
              (:`Update`
                (set `self.fFistRotation` _fistscounterclockwiserotation))
              (:`Finished`
                (set `self.fCurrentFistsRotation` (`self.CurrentFistsRotation`) :!label _label_11)))))
        (:`NewEnumerator3`
          (goto _label_9))))))

(event `StopFistsClockwise`
  ;[1 1 1] TotemRotationLogic
  (`|ExecutionSequence`
    (:`then_0`
      (goto _label_5))
    (:`then_1`
      (goto _label_4 :!via `Stop`))))

(event `StopWingsCounterClockwise`
  ;[1 1 1] TotemRotationLogic
  (`|ExecutionSequence`
    (:`then_0`
      (goto _label_8))
    (:`then_1`
      (goto _label_7 :!via `Stop`))))

(event `StopFistsCounterClockwise`
  ;[1 1 1] TotemRotationLogic
  (`|ExecutionSequence`
    (:`then_0`
      (goto _label_11))
    (:`then_1`
      (goto _label_10 :!via `Stop`))))

(fn `FistsPowerUp`
  (bind (_relativerotation_roll _relativerotation_pitch _relativerotation_yaw) (`KismetMathLibrary.BreakRotator` (`SceneComponent.RelativeRotation` (`self.FistsBase`))))
  (`/Engine/EditorBlueprintResources/StandardMacros.CompareFloat` _relativerotation_yaw
    (:`>`
      (bind _output_get (set `self.fCounterClockwiseBoost` (`KismetMathLibrary.NormalizeToRange` _relativerotation_yaw 0.0 179.0)))
      (if (>= _output_get 0.99)
        (set `self.bAreFistsLocked?` true :!label _label)
        (`self.StopTotemRotation`)))
    (:`<`
      (bind _output_get_2 (set `self.fClockwiseBoost` (- 1.0 (`KismetMathLibrary.NormalizeToRange` _relativerotation_yaw 0.0 -179.0))))
      (if (>= _output_get_2 0.99)
        (goto _label)))))

(fn `OnRep_fCurrentFistsRotation`
  (set `self.bAreFistsTurning?` false))

(fn `OnRep_fCurrentWingsRotation`
  (set `self.bAreWingsTurning?` false))

(fn `OnRep_fEmissive`
  (bind _femissive (`self.fEmissive`))
  (switch `/Game/Core/Data/Enums/E_TotemPart` (`self.eTotemHitPart`)
    (:`NewEnumerator0`
      (`MaterialInstanceDynamic.SetScalarParameterValue` (`self.R_Wing_Material`) "Emissive Intensity" _femissive :!label _label)
      (`MaterialInstanceDynamic.SetScalarParameterValue` (`self.L_Wing_Material`) "Emissive Intensity" _femissive))
    (:`NewEnumerator1`
      (goto _label))
    (:`NewEnumerator2`
      (`MaterialInstanceDynamic.SetScalarParameterValue` (`self.R_Fist_Material`) "Emissive Intensity" _femissive :!label _label_2)
      (`MaterialInstanceDynamic.SetScalarParameterValue` (`self.L_Fist_Material`) "Emissive Intensity" _femissive))
    (:`NewEnumerator3`
      (goto _label_2))
    (:`NewEnumerator4`
      (`MaterialInstanceDynamic.SetScalarParameterValue` (`self.WingBase_Material`) "Emissive Intensity" _femissive))
    (:`NewEnumerator5`
      (`MaterialInstanceDynamic.SetScalarParameterValue` (`self.FistsBase_Material`) "Emissive Intensity" _femissive))
    (:`NewEnumerator6`
      (`MaterialInstanceDynamic.SetScalarParameterValue` (`self.HornsBase_Material`) "Emissive Intensity" _femissive))))

(fn `OnRep_fFistRotation`
  (`SceneComponent.K2_SetRelativeRotation` (`self.FistsBase`) (`KismetMathLibrary.MakeRotator` 0.0 0.0 (+ (* (`self.fFistRotation`) (`self.fTurnAmount`)) (`self.fCurrentFistsRotation`))) false false))

(fn `OnRep_fWingRotation`
  (switch `/Game/Core/Data/Enums/E_TotemRotation` (`self.eTotemRotation`)
    (:`NewEnumerator0`
      (`SceneComponent.K2_SetRelativeRotation` (`self.WingsBase`) (`KismetMathLibrary.MakeRotator` 0.0 0.0 (`self.RotationMaths` (`self.fClockwiseBoost`))) false false))
    (:`NewEnumerator1`
      (`SceneComponent.K2_SetRelativeRotation` (`self.WingsBase`) (`KismetMathLibrary.MakeRotator` 0.0 0.0 (`self.RotationMaths` (`self.fCounterClockwiseBoost`))) false false)
      (`SceneComponent.K2_SetRelativeRotation` (`self.WingsBase`) (`KismetMathLibrary.MakeRotator` 0.0 0.0 (`self.RotationMaths` (`self.fCounterClockwiseBoost`))) false false))))

(fn `ResetEmissive`
  (bind _wingbase_material (`self.WingBase_Material`))
  (bind _earena (`self.eArena`))
  (bind _r_wing_material (`self.R_Wing_Material`))
  (bind _r_fist_material (`self.R_Fist_Material`))
  (bind _r_wing_material_2 (`self.R_Wing_Material`))
  (bind _r_fist_material_2 (`self.R_Fist_Material`))
  (switch `/Game/Core/Data/Enums/E_TotemPart` (`self.eTotemHitPart`)
    (:`NewEnumerator0`
      (switch `/Game/Core/Data/Enums/E_ArenaType` _earena :!label _label
        (:`NewEnumerator0`
          (`MaterialInstanceDynamic.SetScalarParameterValue` _r_wing_material_2 "Emissive Intensity" 0.0)
          (`MaterialInstanceDynamic.SetScalarParameterValue` (`self.L_Wing_Material`) "Emissive Intensity" 0.0)
          (switch `/Game/Core/Data/Enums/E_TotemRotation` (`self.eTotemRotation`)
            (:`NewEnumerator0`
              (`MaterialInstanceDynamic.SetTextureParameterValue` _r_wing_material "Emissive" "/Game/Assets/TikiTandems/Textures/Totem_01/T_Totem_RedMask.T_Totem_RedMask")
              (`MaterialInstanceDynamic.SetTextureParameterValue` (`self.L_Wing_Material`) "Emissive" "/Game/Assets/TikiTandems/Textures/Totem_01/T_Totem_RedMask.T_Totem_RedMask"))
            (:`NewEnumerator1`
              (`MaterialInstanceDynamic.SetTextureParameterValue` _r_wing_material "Emissive" "/Game/Assets/TikiTandems/Textures/Totem_01/T_Totem_BlueMask.T_Totem_BlueMask")
              (`MaterialInstanceDynamic.SetTextureParameterValue` (`self.L_Wing_Material`) "Emissive" "/Game/Assets/TikiTandems/Textures/Totem_01/T_Totem_BlueMask.T_Totem_BlueMask"))))
        (:`NewEnumerator1`
          (`MaterialInstanceDynamic.SetScalarParameterValue` _r_wing_material_2 "Emissive Intensity" 0.0)
          (`MaterialInstanceDynamic.SetScalarParameterValue` (`self.L_Wing_Material`) "Emissive Intensity" 0.0)
          (switch `/Game/Core/Data/Enums/E_TotemRotation` (`self.eTotemRotation`)
            (:`NewEnumerator0`
              (`MaterialInstanceDynamic.SetTextureParameterValue` _r_wing_material "Emissive" "/Game/Assets/TikiTandems/Textures/Totem_02/T_Totem02_PurpleMask.T_Totem02_PurpleMask")
              (`MaterialInstanceDynamic.SetTextureParameterValue` (`self.L_Wing_Material`) "Emissive" "/Game/Assets/TikiTandems/Textures/Totem_02/T_Totem02_PurpleMask.T_Totem02_PurpleMask"))
            (:`NewEnumerator1`
              (`MaterialInstanceDynamic.SetTextureParameterValue` _r_wing_material "Emissive" "/Game/Assets/TikiTandems/Textures/Totem_02/T_Totem02_YellowMask.T_Totem02_YellowMask")
              (`MaterialInstanceDynamic.SetTextureParameterValue` (`self.L_Wing_Material`) "Emissive" "/Game/Assets/TikiTandems/Textures/Totem_02/T_Totem02_YellowMask.T_Totem02_YellowMask"))))))
    (:`NewEnumerator1`
      (goto _label))
    (:`NewEnumerator2`
      (switch `/Game/Core/Data/Enums/E_ArenaType` _earena :!label _label_2
        (:`NewEnumerator0`
          (`MaterialInstanceDynamic.SetScalarParameterValue` _r_fist_material_2 "Emissive Intensity" 0.0)
          (`MaterialInstanceDynamic.SetScalarParameterValue` (`self.L_Fist_Material`) "Emissive Intensity" 0.0)
          (switch `/Game/Core/Data/Enums/E_TotemRotation` (`self.eTotemRotation`)
            (:`NewEnumerator0`
              (`MaterialInstanceDynamic.SetTextureParameterValue` _r_fist_material "Emissive" "/Game/Assets/TikiTandems/Textures/Totem_01/T_Totem_RedMask.T_Totem_RedMask")
              (`MaterialInstanceDynamic.SetTextureParameterValue` (`self.L_Fist_Material`) "Emissive" "/Game/Assets/TikiTandems/Textures/Totem_01/T_Totem_RedMask.T_Totem_RedMask"))
            (:`NewEnumerator1`
              (`MaterialInstanceDynamic.SetTextureParameterValue` _r_fist_material "Emissive" "/Game/Assets/TikiTandems/Textures/Totem_01/T_Totem_BlueMask.T_Totem_BlueMask")
              (`MaterialInstanceDynamic.SetTextureParameterValue` (`self.L_Fist_Material`) "Emissive" "/Game/Assets/TikiTandems/Textures/Totem_01/T_Totem_BlueMask.T_Totem_BlueMask"))))
        (:`NewEnumerator1`
          (`MaterialInstanceDynamic.SetScalarParameterValue` _r_fist_material_2 "Emissive Intensity" 0.0)
          (`MaterialInstanceDynamic.SetScalarParameterValue` (`self.L_Fist_Material`) "Emissive Intensity" 0.0)
          (switch `/Game/Core/Data/Enums/E_TotemRotation` (`self.eTotemRotation`)
            (:`NewEnumerator0`
              (`MaterialInstanceDynamic.SetTextureParameterValue` _r_fist_material "Emissive" "/Game/Assets/TikiTandems/Textures/Totem_02/T_Totem02_PurpleMask.T_Totem02_PurpleMask")
              (`MaterialInstanceDynamic.SetTextureParameterValue` (`self.L_Fist_Material`) "Emissive" "/Game/Assets/TikiTandems/Textures/Totem_02/T_Totem02_PurpleMask.T_Totem02_PurpleMask"))
            (:`NewEnumerator1`
              (`MaterialInstanceDynamic.SetTextureParameterValue` _r_fist_material "Emissive" "/Game/Assets/TikiTandems/Textures/Totem_02/T_Totem02_YellowMask.T_Totem02_YellowMask")
              (`MaterialInstanceDynamic.SetTextureParameterValue` (`self.L_Fist_Material`) "Emissive" "/Game/Assets/TikiTandems/Textures/Totem_02/T_Totem02_YellowMask.T_Totem02_YellowMask"))))))
    (:`NewEnumerator3`
      (goto _label_2))
    (:`NewEnumerator7`
      (`MaterialInstanceDynamic.SetScalarParameterValue` _wingbase_material "Emissive Intensity" 0.0)
      (`MaterialInstanceDynamic.SetTextureParameterValue` _wingbase_material "Emissive" "/Game/Assets/TikiTandems/Textures/Totem_02/Totem_2_Base_EyeMask.Totem_2_Base_EyeMask"))))

(fn `SetTotemStyle`
  (bind _r_fronthit_fists (`self.R_FrontHit_Fists`))
  (bind _l_fronthit_fists (`self.L_FrontHit_Fists`))
  (bind _r_backhit_wings (`self.R_BackHit_Wings`))
  (bind _r_fronthit_wings (`self.R_FrontHit_Wings`))
  (bind _l_fronthit_wings (`self.L_FrontHit_Wings`))
  (bind _l_backhit_fists (`self.L_BackHit_Fists`))
  (bind _r_backhit_fists (`self.R_BackHit_Fists`))
  (bind _l_backhit_wings (`self.L_BackHit_Wings`))
  (switch `/Game/Core/Data/Enums/E_ArenaType` (`self.eArena`)
    (:`NewEnumerator0`
      ;[1 1 1] BasicMaterials Setters and Emissives
      (bind _returnvalue (`PrimitiveComponent.CreateDynamicMaterialInstance` (`self.L_Fist`) 0 null "None"))
      (set `self.L_Fist_Material` _returnvalue)
      (bind _returnvalue_2 (`PrimitiveComponent.CreateDynamicMaterialInstance` (`self.R_Fist`) 0 null "None"))
      (set `self.R_Fist_Material` _returnvalue_2)
      (bind _returnvalue_3 (`PrimitiveComponent.CreateDynamicMaterialInstance` (`self.L_Wing`) 0 null "None"))
      (set `self.L_Wing_Material` _returnvalue_3)
      (bind _returnvalue_4 (`PrimitiveComponent.CreateDynamicMaterialInstance` (`self.R_Wing`) 0 null "None"))
      (set `self.R_Wing_Material` _returnvalue_4)
      (bind _returnvalue_5 (`PrimitiveComponent.CreateDynamicMaterialInstance` (`self.FistsBase`) 0 null "None"))
      (bind _output_get (set `self.FistsBase_Material` _returnvalue_5))
      (`MaterialInstanceDynamic.SetTextureParameterValue` _output_get "Emissive" "/Game/Assets/TikiTandems/Textures/Totem_01/Totem1_Base_EyeMask.Totem1_Base_EyeMask")
      (bind _returnvalue_6 (`PrimitiveComponent.CreateDynamicMaterialInstance` (`self.WingsBase`) 0 null "None"))
      (bind _output_get_2 (set `self.WingBase_Material` _returnvalue_6))
      (`MaterialInstanceDynamic.SetTextureParameterValue` _output_get_2 "Emissive" "/Game/Assets/TikiTandems/Textures/Totem_01/Totem1_Base_EyeMask.Totem1_Base_EyeMask")
      (bind _returnvalue_7 (`PrimitiveComponent.CreateDynamicMaterialInstance` (`self.HornsTotem`) 0 null "None"))
      (bind _output_get_3 (set `self.HornsBase_Material` _returnvalue_7))
      (`MaterialInstanceDynamic.SetTextureParameterValue` _output_get_3 "Emissive" "/Game/Assets/TikiTandems/Textures/Totem_01/Totem1_Base_EyeMask.Totem1_Base_EyeMask"))
    (:`NewEnumerator1`
      (`|ExecutionSequence`
        (:`then_0`
          ;[1 1 1] SetNightTotem Static meshes
          (`StaticMeshComponent.SetStaticMesh` (`self.HornsTotem`) "/Game/Assets/TikiTandems/Meshes/TotemMeshes/SM_HornsTotem02.SM_HornsTotem02")
          (`StaticMeshComponent.SetStaticMesh` (`self.TotemBase`) "/Game/Assets/TikiTandems/Meshes/TotemMeshes/SM_BaseTotem02.SM_BaseTotem02")
          (`StaticMeshComponent.SetStaticMesh` (`self.WingsBase`) "/Game/Assets/TikiTandems/Meshes/TotemMeshes/SM_WingsBase_02.SM_WingsBase_02")
          (`StaticMeshComponent.SetStaticMesh` (`self.R_Wing`) "/Game/Assets/TikiTandems/Meshes/TotemMeshes/SM_R_Wing_02.SM_R_Wing_02")
          (`StaticMeshComponent.SetStaticMesh` (`self.L_Wing`) "/Game/Assets/TikiTandems/Meshes/TotemMeshes/SM_L_Wing_02.SM_L_Wing_02")
          (`StaticMeshComponent.SetStaticMesh` (`self.FistsBase`) "/Game/Assets/TikiTandems/Meshes/TotemMeshes/SM_FistsTotem02.SM_FistsTotem02")
          (`StaticMeshComponent.SetStaticMesh` (`self.R_Fist`) "/Game/Assets/TikiTandems/Meshes/TotemMeshes/SM_R_Fist_02.SM_R_Fist_02")
          (`StaticMeshComponent.SetStaticMesh` (`self.L_Fist`) "/Game/Assets/TikiTandems/Meshes/TotemMeshes/SM_L_Fist_02.SM_L_Fist_02"))
        (:`then_1`
          ;[1 1 1] Set materials for Night totem
          (bind _returnvalue_8 (`PrimitiveComponent.CreateDynamicMaterialInstance` (`self.R_Wing`) 0 "/Game/Assets/TikiTandems/Materials/Instances/MI_Totem_02_Marked.MI_Totem_02_Marked" "None"))
          (set `self.R_Wing_Material` _returnvalue_8)
          (bind _returnvalue_9 (`PrimitiveComponent.CreateDynamicMaterialInstance` (`self.L_Wing`) 0 "/Game/Assets/TikiTandems/Materials/Instances/MI_Totem_02_Marked.MI_Totem_02_Marked" "None"))
          (set `self.L_Wing_Material` _returnvalue_9)
          (bind _returnvalue_10 (`PrimitiveComponent.CreateDynamicMaterialInstance` (`self.R_Fist`) 0 "/Game/Assets/TikiTandems/Materials/Instances/MI_Totem_02_Marked.MI_Totem_02_Marked" "None"))
          (set `self.R_Fist_Material` _returnvalue_10)
          (bind _returnvalue_11 (`PrimitiveComponent.CreateDynamicMaterialInstance` (`self.L_Fist`) 0 "/Game/Assets/TikiTandems/Materials/Instances/MI_Totem_02_Marked.MI_Totem_02_Marked" "None"))
          (set `self.L_Fist_Material` _returnvalue_11)
          (bind _returnvalue_12 (`PrimitiveComponent.CreateDynamicMaterialInstance` (`self.WingsBase`) 0 "/Game/Assets/TikiTandems/Materials/Instances/MI_Totem_02_Marked.MI_Totem_02_Marked" "None"))
          (bind _output_get_4 (set `self.WingBase_Material` _returnvalue_12))
          (`MaterialInstanceDynamic.SetTextureParameterValue` _output_get_4 "Emissive" "/Game/Assets/TikiTandems/Textures/Totem_02/Totem_2_Base_EyeMask.Totem_2_Base_EyeMask")
          (bind _returnvalue_13 (`PrimitiveComponent.CreateDynamicMaterialInstance` (`self.FistsBase`) 0 "/Game/Assets/TikiTandems/Materials/Instances/MI_Totem_02_Marked.MI_Totem_02_Marked" "None"))
          (bind _output_get_5 (set `self.FistsBase_Material` _returnvalue_13))
          (`MaterialInstanceDynamic.SetTextureParameterValue` _output_get_5 "Emissive" "/Game/Assets/TikiTandems/Textures/Totem_02/Totem_2_Base_EyeMask.Totem_2_Base_EyeMask")
          (bind _returnvalue_14 (`PrimitiveComponent.CreateDynamicMaterialInstance` (`self.HornsTotem`) 0 "/Game/Assets/TikiTandems/Materials/Instances/MI_Totem_02_Marked.MI_Totem_02_Marked" "None"))
          (bind _output_get_6 (set `self.HornsBase_Material` _returnvalue_14))
          (`MaterialInstanceDynamic.SetTextureParameterValue` _output_get_6 "Emissive" "/Game/Assets/TikiTandems/Textures/Totem_02/Totem_2_Base_EyeMask.Totem_2_Base_EyeMask"))
        (:`then_2`
          ;[1 1 1] SetRelativeLocation for static meshes
          (`SceneComponent.K2_SetRelativeLocation` _r_backhit_fists (- (`SceneComponent.RelativeLocation` _r_backhit_fists) (0.0 0.0 100.0)) false false)
          (`SceneComponent.K2_SetRelativeLocation` _r_fronthit_fists (- (`SceneComponent.RelativeLocation` _r_fronthit_fists) (0.0 0.0 100.0)) false false)
          (`SceneComponent.K2_SetRelativeLocation` _l_fronthit_fists (- (`SceneComponent.RelativeLocation` _l_fronthit_fists) (0.0 0.0 100.0)) false false)
          (`SceneComponent.K2_SetRelativeLocation` _r_backhit_wings (- (`SceneComponent.RelativeLocation` _r_backhit_wings) (0.0 0.0 100.0)) false false)
          (`SceneComponent.K2_SetRelativeLocation` _r_fronthit_wings (- (`SceneComponent.RelativeLocation` _r_fronthit_wings) (0.0 0.0 100.0)) false false)
          (`SceneComponent.K2_SetRelativeLocation` _l_fronthit_wings (- (`SceneComponent.RelativeLocation` _l_fronthit_wings) (0.0 0.0 100.0)) false false)
          (`SceneComponent.K2_SetRelativeLocation` _l_backhit_fists (- (`SceneComponent.RelativeLocation` _l_backhit_fists) (0.0 0.0 100.0)) false false)
          (`SceneComponent.K2_SetRelativeLocation` _l_backhit_wings (- (`SceneComponent.RelativeLocation` _l_backhit_wings) (0.0 0.0 100.0)) false false))))))

(fn `StopTotemRotation`
  (switch `/Game/Core/Data/Enums/E_TotemPart` (`self.eTotemHitPart`)
    (:`NewEnumerator0`
      (if (`self.bAreWingsTurning?`) :!label _label
        (`self.StopTurningWings`)
        (set `self.bAreWingsTurning?` false)))
    (:`NewEnumerator1`
      (goto _label))
    (:`NewEnumerator2`
      (if (`self.bAreFistsTurning?`) :!label _label_2
        (`self.StopTurningFists`)
        (set `self.bAreFistsTurning?` false)))
    (:`NewEnumerator3`
      (goto _label_2))))

(fn `TotemRotation`
  (switch `/Game/Core/Data/Enums/E_TotemPart` (`self.eTotemHitPart`)
    (:`NewEnumerator0`
      ;[1 1 1] LeftWing
      (`/Engine/EditorBlueprintResources/StandardMacros.CompareFloat` (`KismetMathLibrary.Vector_Distance` (`self.vHitLocation`) (`SceneComponent.K2_GetComponentLocation` (`self.L_FrontHit_Wings`))) (`KismetMathLibrary.Vector_Distance` (`self.vHitLocation`) (`SceneComponent.K2_GetComponentLocation` (`self.L_BackHit_Wings`)))
        (:`>`
          (set `self.eTotemRotation` "NewEnumerator1"))
        (:`<`
          (set `self.eTotemRotation` "NewEnumerator0"))))
    (:`NewEnumerator1`
      ;[1 1 1] RightWing
      (`/Engine/EditorBlueprintResources/StandardMacros.CompareFloat` (`KismetMathLibrary.Vector_Distance` (`self.vHitLocation`) (`SceneComponent.K2_GetComponentLocation` (`self.R_FrontHit_Wings`))) (`KismetMathLibrary.Vector_Distance` (`self.vHitLocation`) (`SceneComponent.K2_GetComponentLocation` (`self.R_BackHit_Wings`)))
        (:`>`
          (set `self.eTotemRotation` "NewEnumerator0"))
        (:`<`
          (set `self.eTotemRotation` "NewEnumerator1"))))
    (:`NewEnumerator2`
      ;[1 1 1] LeftFist
      (`/Engine/EditorBlueprintResources/StandardMacros.CompareFloat` (`KismetMathLibrary.Vector_Distance` (`self.vHitLocation`) (`SceneComponent.K2_GetComponentLocation` (`self.L_FrontHit_Fists`))) (`KismetMathLibrary.Vector_Distance` (`self.vHitLocation`) (`SceneComponent.K2_GetComponentLocation` (`self.L_BackHit_Fists`)))
        (:`>`
          (set `self.eTotemRotation` "NewEnumerator1"))
        (:`<`
          (set `self.eTotemRotation` "NewEnumerator0"))))
    (:`NewEnumerator3`
      ;[1 1 1] RightWing
      (`/Engine/EditorBlueprintResources/StandardMacros.CompareFloat` (`KismetMathLibrary.Vector_Distance` (`self.vHitLocation`) (`SceneComponent.K2_GetComponentLocation` (`self.R_FrontHit_Fists`))) (`KismetMathLibrary.Vector_Distance` (`self.vHitLocation`) (`SceneComponent.K2_GetComponentLocation` (`self.R_BackHit_Fists`)))
        (:`>`
          (set `self.eTotemRotation` "NewEnumerator0"))
        (:`<`
          (set `self.eTotemRotation` "NewEnumerator1"))))
    (:`NewEnumerator7`
      (set `self.eTotemRotation` "NewEnumerator2"))))

(fn `UserConstructionScript`)

(fn `WhichTotemPart`
  (bind _hittotempart (`self.HitTotemPart`))
  (if (== (`self.L_Wing`) _hittotempart)
    (set `self.eTotemHitPart` "NewEnumerator0")
    (elif (== (`self.R_Wing`) _hittotempart)
      (set `self.eTotemHitPart` "NewEnumerator1")
      (elif (== (`self.L_Fist`) _hittotempart)
        (set `self.eTotemHitPart` "NewEnumerator2")
        (elif (== (`self.R_Fist`) _hittotempart)
          (set `self.eTotemHitPart` "NewEnumerator3")
          (elif (== (`self.WingsBase`) _hittotempart)
            (set `self.eTotemHitPart` "NewEnumerator4")
            (elif (== (`self.FistsBase`) _hittotempart)
              (set `self.eTotemHitPart` "NewEnumerator5")
              (elif (== (`self.HornsTotem`) _hittotempart)
                (set `self.eTotemHitPart` "NewEnumerator6")
                (else
                  (set `self.eTotemHitPart` "NewEnumerator7")))))))))
  (return))