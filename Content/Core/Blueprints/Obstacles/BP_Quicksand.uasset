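; Quicksand arena obstacle that slows and visually sinks a BP_Tiki character standing in it.
; On game start, a random roll decides whether a flip-flopped timeline raises or lowers the initially buried decal, rerolling after a random delay.
; Overlap starts a looping timer that gradually cuts walk speed and lowers the mesh to set limits.
; Leaving clears the timer and restores speed and mesh position.
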(event `self.ReceiveBeginPlay`
  (`SceneComponent.K2_SetRelativeLocation` (`self.Decal`) (0.0 0.0 -250.0) false false)
  (bind _asgm_arena (cast `/Game/Core/Blueprints/GameRules/GameModes/GM_Arena` (`GameplayStatics.GetGameMode`)))
  (add `/Game/Core/Blueprints/GameRules/GameModes/GM_Arena.StartGame` _asgm_arena (delegate `RandomizeQuicksands`)))

(event `RandomizeQuicksands`
  (if (`KismetMathLibrary.RandomBool`)
    (`/Engine/EditorBlueprintResources/StandardMacros.FlipFlop`
      (:`A`
        (bind (_direction _zmovement) (`Timeline|MoveUpOrDown` :!via `PlayFromStart` :!label _label)
          (:`Update`
            (`SceneComponent.K2_SetRelativeLocation` (`self.Decal`) (`KismetMathLibrary.MakeVector` 0.0 0.0 _zmovement) false false))
          (:`Finished`
            (`KismetSystemLibrary.Delay` (`KismetMathLibrary.RandomFloatInRange` 10.0 20.0))
            (`self.RandomizeQuicksands`))))
      (:`B`
        (goto _label :!via `ReverseFromEnd`)))))

(event `self.Collision.OnComponentBeginOverlap`
  (params (OverlappedComponent :type "PrimitiveComponent Object Reference") (OtherActor :type "Actor Object Reference") (OtherComp :type "PrimitiveComponent Object Reference") (OtherBodyIndex :type Integer) (bFromSweep :type Boolean) (SweepResult :type "HitResult Structure (by ref)"))
  (bind _asbp_tiki (cast `/Game/Core/Blueprints/TikiCharacter/Blueprint/BP_Tiki` OtherActor))
  (bind _output_get (set `self.BPTikiReference` _asbp_tiki))
  (set `self.DefaultWalkSpeed` (`CharacterMovementComponent.MaxWalkSpeed` (`Character.CharacterMovement` _output_get)))
  (bind _returnvalue (`KismetSystemLibrary.K2_SetTimerDelegate` (delegate `SlowDownPlayer`) 0.05 true)))

(event `SlowDownPlayer`
  (bind _bptikireference (`self.BPTikiReference`))
  (bind _charactermovement (`Character.CharacterMovement` _bptikireference))
  (bind _mesh (`Character.Mesh` _bptikireference))
  (bind (_relativelocation_x _relativelocation_y _relativelocation_z) (`KismetMathLibrary.BreakVector` (`SceneComponent.RelativeLocation` _mesh)))
  (set `CharacterMovementComponent.MaxWalkSpeed` (`KismetMathLibrary.FClamp` (* (`CharacterMovementComponent.MaxWalkSpeed` _charactermovement) 0.93) 150.0 1000.0) _charactermovement)
  (if (not (< _relativelocation_z -90.0))
    (`SceneComponent.K2_AddLocalOffset` _mesh (0.0 0.0 -0.4) false false)))

(event `self.Collision.OnComponentEndOverlap`
  (params (OverlappedComponent :type "PrimitiveComponent Object Reference") (OtherActor :type "Actor Object Reference") (OtherComp :type "PrimitiveComponent Object Reference") (OtherBodyIndex :type Integer))
  (bind _asbp_tiki (cast `/Game/Core/Blueprints/TikiCharacter/Blueprint/BP_Tiki` OtherActor))
  (set `CharacterMovementComponent.MaxWalkSpeed` (`self.DefaultWalkSpeed`) (`Character.CharacterMovement` _asbp_tiki))
  (`KismetSystemLibrary.K2_ClearAndInvalidateTimerHandle` (stale `self.Collision.OnComponentBeginOverlap` _returnvalue))
  (`SceneComponent.K2_SetRelativeLocation` (`Character.Mesh` (`self.BPTikiReference`)) (0.0 0.0 -70.0) false false))

(fn `UserConstructionScript`)