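; BP_Geiser is a geyser obstacle that launches an overlapping BP_Tiki upward and forward when ready, also setting its gravity scale.
; Timelines scale the mesh and splash through a self-restarting idle, shooting and inactive cycle gated by the Ready flag.
; After shooting, it strips its effects, light and water plane, then restores them after FGeiserTimer with a camera shake and wake-up animation.
; The pre-wake jitter timeline multiplies its offset by zero, so the actor stays put.
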(event `GeiserInactive`
  ;[1 1 1] Geiser Inactive logic
  (`self.DisableVisuals`)
  (`|ExecutionSequence`
    (:`then_0`
      (bind (_direction _inactivetimer) (`Timeline|InactiveGeiserTimeline` :!via `PlayFromStart`)
        (:`Update`
          (`SceneComponent.SetRelativeScale3D` (`self.Geiser`) (`KismetMathLibrary.Conv_DoubleToVector` _inactivetimer)))))
    (:`then_1`
      (`KismetSystemLibrary.Delay` (`self.fGeiserTimer`))
      (`self.ActivateVisuals`)
      (`GameplayStatics.PlayWorldCameraShake` "/Game/Core/Cinematics/CameraShake/BP_SpearCage_CS.BP_SpearCage_CS_C" (`self.K2_GetActorLocation`) 500.0 1500.0)
      (bind (_direction_2 _zscalegeiser) (`Timeline|GeiserWakeUpTimeline`)
        (:`Update`
          (`SceneComponent.SetRelativeScale3D` (`self.Geiser`) (`KismetMathLibrary.MakeVector` 1.0 1.0 _zscalegeiser)))
        (:`Finished`
          (set `self.bReady?` true)
          (`self.GeiserIdleAnimation`))))
    (:`then_2`
      (`KismetSystemLibrary.Delay` (- (`self.fGeiserTimer`) 1.0))
      (bind (_direction_3 _offset) (`Timeline|GeiserJitterTimeline`)
        (:`Update`
          (bind _returnvalue (* _offset 0.0))
          (`self.K2_SetActorLocation` (+ (`KismetMathLibrary.MakeVector` _returnvalue _returnvalue) (`self.K2_GetActorLocation`))))))))

(event `GeiserShoot`
  ;[1 1 1] Geiser shooting/active logic
  (set `self.bReady?` false)
  (`ActorComponent.Activate` (`self.WaterSplashFX`) false)
  (`self.StopAnimation`)
  (bind (_direction _zscalegeiser _zscaleparticles) (`Timeline|ShootingAnimationTimeline` :!via `PlayFromStart`)
    (:`Update`
      (`SceneComponent.SetRelativeScale3D` (`self.Geiser`) (`KismetMathLibrary.MakeVector` 1.0 1.0 _zscalegeiser))
      (`SceneComponent.SetRelativeScale3D` (`self.WaterSplashFX`) (`KismetMathLibrary.MakeVector` 0.7 0.7 _zscaleparticles)))
    (:`Finished`
      (`self.GeiserInactive`))))

(event `GeiserIdleAnimation`
  (bind _plane (`self.Plane`))
  (bind (_relativelocation_x _relativelocation_y) (`KismetMathLibrary.BreakVector` (`SceneComponent.RelativeLocation` _plane)))
  ;[1 1 1] Geiser idle animation logic
  (if (`self.bReady?`)
    (bind (_direction _zscale _zwaterlocation) (`Timeline|IdleAnimationTimeline` :!via `PlayFromStart` :!label _label)
      (:`Update`
        (`SceneComponent.SetRelativeScale3D` (`self.Geiser`) (`KismetMathLibrary.MakeVector` 1.0 1.0 _zscale))
        (`SceneComponent.K2_SetRelativeLocation` _plane (`KismetMathLibrary.MakeVector` _relativelocation_x _relativelocation_y _zwaterlocation) false false))
      (:`Finished`
        (`self.GeiserIdleAnimation`)))))

(event `StopAnimation`
  ;[1 1 1] Geiser idle animation logic
  (goto _label :!via `Stop`))

(event `self.Collision.OnComponentBeginOverlap`
  (params (OverlappedComponent :type "PrimitiveComponent Object Reference") (OtherActor :type "Actor Object Reference") (OtherComp :type "PrimitiveComponent Object Reference") (OtherBodyIndex :type Integer) (bFromSweep :type Boolean) (SweepResult :type "HitResult Structure (by ref)"))
  ;[1 1 1] BeginPlay and Collision logic
  (if (`self.bReady?`)
    (`self.GeiserShoot`)
    (bind _asbp_tiki (cast `/Game/Core/Blueprints/TikiCharacter/Blueprint/BP_Tiki` OtherActor))
    (bind _charactermovement (`Character.CharacterMovement` _asbp_tiki))
    (set `MovementComponent.Velocity` (0.0 0.0 0.0) _charactermovement)
    (bind (_returnvalue_x _returnvalue_y) (`KismetMathLibrary.BreakVector` (* (`self.GetActorForwardVector` _asbp_tiki) (800.0 800.0 1.0))))
    (`Character.LaunchCharacter` _asbp_tiki (`KismetMathLibrary.MakeVector` _returnvalue_x _returnvalue_y (`self.fGeiserStrength`)) false false)
    (set `CharacterMovementComponent.GravityScale` 3.0 _charactermovement)))

(event `self.ReceiveBeginPlay`
  ;[1 1 1] BeginPlay and Collision logic
  (`self.GeiserIdleAnimation`))

(fn `ActivateVisuals`
  (`NiagaraComponent.SetAsset` (`self.BubblesFX`) "/Game/Assets/VFX/Custom/NS_Bubbles.NS_Bubbles" true)
  (`NiagaraComponent.SetAsset` (`self.WaterSplashFX`) "/Game/Assets/VFX/Flipbook_VFX/Shared/Particles/Water/NS_Water_MainSplash_02.NS_Water_MainSplash_02" true)
  (`LightComponent.SetIntensity` (`self.PointLight`) 25000.0)
  (`StaticMeshComponent.SetStaticMesh` (`self.Plane`) "/Engine/BasicShapes/Plane.Plane"))

(fn `DisableVisuals`
  (`NiagaraComponent.SetAsset` (`self.WaterSplashFX`) null true)
  (`NiagaraComponent.SetAsset` (`self.BubblesFX`) null true)
  (`LightComponent.SetIntensity` (`self.PointLight`) 0.0)
  (`StaticMeshComponent.SetStaticMesh` (`self.Plane`) null))

(fn `UserConstructionScript`)