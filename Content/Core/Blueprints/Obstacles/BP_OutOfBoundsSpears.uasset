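; An out-of-bounds spear obstacle that strikes the Tiki character when it overlaps the collision.
; On overlap, the SpearHit timeline animates the spear mesh's Z scale while its X and Y stay fixed.
; After a short delay, it zeroes the Tiki's movement velocity and applies damage with the DT_Launch damage type, leaving any response to that type outside this Blueprint.
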(event `self.Collision.OnComponentBeginOverlap`
  (params (OverlappedComponent :type "PrimitiveComponent Object Reference") (OtherActor :type "Actor Object Reference") (OtherComp :type "PrimitiveComponent Object Reference") (OtherBodyIndex :type Integer) (bFromSweep :type Boolean) (SweepResult :type "HitResult Structure (by ref)"))
  (bind _asbp_tiki (cast `/Game/Core/Blueprints/TikiCharacter/Blueprint/BP_Tiki` OtherActor))
  (`|ExecutionSequence`
    (:`then_0`
      (bind (_direction _spearhit) (`Timeline|SpearHit` :!via `PlayFromStart`)
        (:`Update`
          (`SceneComponent.SetRelativeScale3D` (`self.Spear`) (`KismetMathLibrary.MakeVector` 2.25 2.25 _spearhit)))))
    (:`then_1`
      (`KismetSystemLibrary.Delay` 0.08)
      (bind _charactermovement (`Character.CharacterMovement` _asbp_tiki))
      (`/Engine/EditorBlueprintResources/StandardMacros.IsValid` _charactermovement
        (:`Is Valid`
          (set `MovementComponent.Velocity` (0.0 0.0 0.0) _charactermovement)
          (`GameplayStatics.ApplyDamage` _asbp_tiki 0.5 null self "/Game/Core/Data/DamageTypes/DT_Launch.DT_Launch_C"))))))

(fn `UserConstructionScript`)