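; Player controller for local two-player character selection, taking each player from joining through character lock to day/night arena choice and match start.
; A MultiGate on IA_Next stages the flow: claim a selection actor, toggle lock, start.
; RepNotifies swap input mapping contexts on lock and store the chosen class by controller ID in GI_TikiTandems.
; Once both lock, previous/next input toggles sky and light, with only the widget owner keeping input.
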(event `self.ReceiveBeginPlay`
  ;[1 1 1] Event BeginPlay
  (`WidgetBlueprintLibrary.SetInputMode_GameOnly` self)
  (set `self.iIndex` 0)
  (`KismetSystemLibrary.Delay` 1.2)
  (`self.EnableInput` self self))

(event `EnhancedInput|/Game/Core/Blueprints/Input/InputActions/IA_NextSelection`
  (params (ActionValue :type Boolean) (ElapsedSeconds :type "Float (double-precision)") (TriggeredSeconds :type "Float (double-precision)") (InputAction :type "InputAction Object Reference" :default "/Game/Core/Blueprints/Input/InputActions/IA_NextSelection.IA_NextSelection"))
  ;[1 1 1] Character and map switching logic
  (:`Started`
    (set `self.bNextPrevious` true)
    (if (`self.bArenaLock?`) :!label _label
      (bind _returnvalue (`GameplayStatics.GetActorOfClass` "/Script/Engine.DirectionalLight"))
      (bind _asgi_tiki_tandems (cast `/Game/Core/Blueprints/GameRules/GI_TikiTandems` (`GameplayStatics.GetGameInstance`)))
      (`/Engine/EditorBlueprintResources/StandardMacros.FlipFlop`
        (:`A`
          (`self.SetNightArena`)
          (set `/Game/Core/Blueprints/GameRules/GI_TikiTandems.eArenaType` "NewEnumerator1" _asgi_tiki_tandems)
          (bind (_direction _shiftdaynight) (`Timeline|Timeline` :!label _label_2)
            (:`Update`
              (bind _lightcomponent (`Light.LightComponent` _returnvalue))
              (`/Engine/EditorBlueprintResources/StandardMacros.IsValid` _lightcomponent
                (:`Is Valid`
                  (`LightComponent.SetIntensity` _lightcomponent _shiftdaynight))))))
        (:`B`
          (`self.SetDayArena`)
          (set `/Game/Core/Blueprints/GameRules/GI_TikiTandems.eArenaType` "NewEnumerator0" _asgi_tiki_tandems)
          (goto _label_2 :!via `Reverse`)))
      (else
        (`self.SwitchCharacter` (`self.bNextPrevious`) (`self.PlayerActor`))))))

(event `EnhancedInput|/Game/Core/Blueprints/Input/InputActions/IA_PreviousSelection`
  (params (ActionValue :type Boolean) (ElapsedSeconds :type "Float (double-precision)") (TriggeredSeconds :type "Float (double-precision)") (InputAction :type "InputAction Object Reference" :default "/Game/Core/Blueprints/Input/InputActions/IA_PreviousSelection.IA_PreviousSelection"))
  ;[1 1 1] Character and map switching logic
  (:`Started`
    (set `self.bNextPrevious` false)
    (goto _label)))

(event `EnablePlayer`
  ;[1 1 1] Enable player input
  (`self.SetActorHiddenInGame` (`self.PlayerActor`) false)
  (`self.SetActorHiddenInGame` (`self.PlayerClassName`) false)
  (`/Game/Core/Blueprints/Functions/BFL_General.AddInputMappingContext` self "/Game/Core/Blueprints/Input/InputActionMappings/IMC_CharacterSelection.IMC_CharacterSelection"))

(event `EnhancedInput|/Game/Core/Blueprints/Input/InputActions/IA_Exit`
  (params (ActionValue :type Boolean) (ElapsedSeconds :type "Float (double-precision)") (TriggeredSeconds :type "Float (double-precision)") (InputAction :type "InputAction Object Reference" :default "/Game/Core/Blueprints/Input/InputActions/IA_Exit.IA_Exit"))
  ;[1 1 1] ExitGame
  (:`Started`
    (`GameplayStatics.OpenLevelBySoftObjectPtr` "/Game/maps/L_MainMenu.L_MainMenu")))

(event `ChooseArena`
  (bind _characterselectionref (`self.CharacterSelectionRef`))
  ;[1 1 1] Set arena widget logic
  (`/Engine/EditorBlueprintResources/StandardMacros.IsValid` _characterselectionref
    (:`Is Valid`
      (if (== (`self.iPlayerIndex`) (`self.iWidgetOwner`))
        (`/Game/Core/Widgets/CharacterSelection/W_CharacterSelectionScreen.ChooseArena` _characterselectionref true)
        (`/Game/Core/Blueprints/Functions/BFL_General.AddInputMappingContext` self "/Game/Core/Blueprints/Input/InputActionMappings/IMC_CharacterSelection.IMC_CharacterSelection")
        (`/Game/Core/Blueprints/Functions/BFL_General.RemoveInputMappingContext` self "/Game/Core/Blueprints/Input/InputActionMappings/IMC_Lock.IMC_Lock")
        (else
          (`/Game/Core/Blueprints/Functions/BFL_General.RemoveAllInputMappingContexts` self :!label _label_3))))
    (:`Is Not Valid`
      (goto _label_3))))

(event `SetPlayerClass`
  (bind _asgi_tiki_tandems (cast `/Game/Core/Blueprints/GameRules/GI_TikiTandems` (`GameplayStatics.GetGameInstance`) :!pure true))
  ;[1 1 1] SetPlayerClass in GI logic
  (bind _characterclass (`self.GetPlayerCharacterClass` (`self.eSelectedCharacter`)))
  (`BlueprintMapLibrary.Map_Add` (`/Game/Core/Blueprints/GameRules/GI_TikiTandems.PlayerClassByID` _asgi_tiki_tandems) (`BlueprintMapLibrary.Map_Find` (`/Game/Core/Blueprints/GameRules/GI_TikiTandems.ControllerID` _asgi_tiki_tandems) (`GameplayStatics.GetPlayerControllerID` self)) _characterclass))

(event `EnhancedInput|/Game/Core/Blueprints/Input/InputActions/IA_Next`
  (params (ActionValue :type Boolean) (ElapsedSeconds :type "Float (double-precision)") (TriggeredSeconds :type "Float (double-precision)") (InputAction :type "InputAction Object Reference" :default "/Game/Core/Blueprints/Input/InputActions/IA_Next.IA_Next"))
  ;[1 1 1] Lock character and arena logic
  (:`Started`
    (`|MultiGate` false false (`self.iIndex`) :!label _label_4
      (:`Out 0`
        (bind _outactors (`GameplayStatics.GetAllActorsOfClass` "/Game/Core/Blueprints/Characters/CharacterSelector/BP_CharacterSelection.BP_CharacterSelection_C"))
        (for (_array_element _array_index) _outactors :!label _label_5
          (if (not (`/Game/Core/Blueprints/Characters/CharacterSelector/BP_CharacterSelection.bIsTaken?` _array_element))
            (set `self.PlayerActor` _array_element)
            (set `/Game/Core/Blueprints/Characters/CharacterSelector/BP_CharacterSelection.bIsTaken?` true _array_element)
            (if (== _array_index 0)
              (bind _asgm_character_selection_local (cast `/Game/Core/Blueprints/GameRules/GameModes/GM_CharacterSelection_Local` (`GameplayStatics.GetGameMode`)))
              (`Widget.RemoveFromParent` (`/Game/Core/Blueprints/GameRules/GameModes/GM_CharacterSelection_Local.wCharacterSelection` _asgm_character_selection_local))
              (`self.CreateWidgets`)
              (`Widget.SetVisibility` (`/Game/Core/Widgets/CharacterSelection/W_CharacterSelectionScreen.WaitingP1` (`self.CharacterSelectionRef`)) "Hidden")
              (else
                (`Widget.SetVisibility` (`/Game/Core/Widgets/CharacterSelection/W_CharacterSelectionScreen.WaitingP2` (`/Game/Core/Blueprints/Input/Controllers/BPC_CharacterSelection_Local.CharacterSelectionRef` (cast `/Game/Core/Blueprints/Input/Controllers/BPC_CharacterSelection_Local` (`GameplayStatics.GetPlayerController` (`self.iWidgetOwner`)) :!pure true))) "Hidden")))
            (bind _asgi_tiki_tandems (cast `/Game/Core/Blueprints/GameRules/GI_TikiTandems` (`GameplayStatics.GetGameInstance`)))
            (`BlueprintMapLibrary.Map_Add` (`/Game/Core/Blueprints/GameRules/GI_TikiTandems.ControllerID` _asgi_tiki_tandems) (`GameplayStatics.GetPlayerControllerID` self) _array_index)
            (`self.Break`)
            (`KismetSystemLibrary.Delay` 0.2)
            (`self.InitializeSelectorData`)
            (`self.EnablePlayer`)
            (`self.SetPlayerClass`))))
      (:`Out 1`
        (`/Game/Core/Blueprints/Characters/CharacterSelector/BP_CharacterSelection.LockCharacter` (`self.PlayerActor`) (`self.PlayerClassName`))
        (set `self.iIndex` 1)
        (`self.ResetGate`)
        (if (`self.IsServer?`)
          (`/Engine/EditorBlueprintResources/StandardMacros.FlipFlop`
            (:`A`
              (set `self.P1Locked?` true)
              (`KismetSystemLibrary.K2_SetTimerDelegate` (delegate `CheckIfReady`) 0.1 :!label _label_6))
            (:`B`
              (set `self.P1Locked?` false)))
          (else
            (`/Engine/EditorBlueprintResources/StandardMacros.FlipFlop`
              (:`A`
                (set `self.P2Locked?` true)
                (goto _label_6))
              (:`B`
                (set `self.P2Locked?` false))))))
      (:`Out 2`
        (`self.StartGame`)
        (`KismetSystemLibrary.Delay` 1.5)
        (bind _asgm_character_selection_local_2 (cast `/Game/Core/Blueprints/GameRules/GameModes/GM_CharacterSelection_Local` (`GameplayStatics.GetGameMode`)))
        (`/Game/Core/Blueprints/GameRules/GameModes/GM_CharacterSelection_Local.ShowLoadingScreen` _asgm_character_selection_local_2)))))

(event `Break`
  ;[1 1 1] Lock character and arena logic
  (goto _label_5 :!via `Break`))

(event `ResetGate`
  ;[1 1 1] Lock character and arena logic
  (goto _label_4 :!via `Reset`))

(event `CheckIfReady`
  ;[1 1 1] Lock character and arena logic
  (bind _outactors (`GameplayStatics.GetAllActorsOfClass` "/Game/Core/Blueprints/Characters/CharacterSelector/BP_CharacterSelection.BP_CharacterSelection_C"))
  (for _array_element _outactors
    (if (`/Game/Core/Blueprints/Characters/CharacterSelector/BP_CharacterSelection.bIsLocked?` _array_element)
      (`/Engine/EditorBlueprintResources/StandardMacros.IncrementInt` (`self.iCounter`))))
  (if (== (`self.iCounter`) 2)
    (for _array_element_2 (`/Game/Core/Blueprints/GameRules/GameModes/GM_CharacterSelection_Local.PlayerControllers` (cast `/Game/Core/Blueprints/GameRules/GameModes/GM_CharacterSelection_Local` (`GameplayStatics.GetGameMode`) :!pure true))
      (bind _asbpc_character_selection_local (cast `/Game/Core/Blueprints/Input/Controllers/BPC_CharacterSelection_Local` _array_element_2 :!pure true))
      (`self.SelectArena` _asbpc_character_selection_local)
      (set `/Game/Core/Blueprints/Input/Controllers/BPC_CharacterSelection_Local.bArenaLock?` true _asbpc_character_selection_local))
    (else
      (set `self.iCounter` 0))))

(fn `CreateWidgets`
  (bind _returnvalue (`|CreateWidget` "/Game/Core/Widgets/CharacterSelection/W_CharacterSelectionScreen.W_CharacterSelectionScreen_C" self))
  (bind _output_get (set `self.CharacterSelectionRef` _returnvalue))
  (`UserWidget.AddToViewport` _output_get 0)
  (bind _asgm_character_selection_local (cast `/Game/Core/Blueprints/GameRules/GameModes/GM_CharacterSelection_Local` (`GameplayStatics.GetGameMode`)))
  (for _array_element (`/Game/Core/Blueprints/GameRules/GameModes/GM_CharacterSelection_Local.PlayerControllers` _asgm_character_selection_local)
    (bind _asbpc_character_selection_local (cast `/Game/Core/Blueprints/Input/Controllers/BPC_CharacterSelection_Local` _array_element))
    (set `/Game/Core/Blueprints/Input/Controllers/BPC_CharacterSelection_Local.iWidgetOwner` (`GameplayStatics.GetPlayerControllerID` self) _asbpc_character_selection_local)
    (return)))

(fn `GetPlayerCharacterClass`
  (params (CharacterSelection :type "/Game/Core/Data/Enums/E_CharacterClasses Enum" :default "NewEnumerator0"))
  (returns (CharacterClass :type "/Game/Core/Blueprints/TikiCharacter/Blueprint/BP_Tiki Class Reference"))
  (switch `/Game/Core/Data/Enums/E_CharacterClasses` CharacterSelection
    (:`NewEnumerator0`
      (return "/Game/Core/Blueprints/Characters/Spearman/BP_Spearman.BP_Spearman_C"))
    (:`NewEnumerator1`
      (return "/Game/Core/Blueprints/Characters/Bonkerman/BP_Bonkerman.BP_Bonkerman_C"))
    (:`NewEnumerator2`
      (return "/Game/Core/Blueprints/Characters/Magicman/BP_Magicman.BP_Magicman_C"))))

(fn `InitializeSelectorData`
  (bind _outactors (`GameplayStatics.GetAllActorsOfClass` "/Game/Core/Widgets/MainMenu/W_WorldButton.W_WorldButton_C"))
  (for _array_element _outactors
    (if (`self.Check` (`Actor.Tags` _array_element))
      (set `self.PlayerClassName` _array_element)
      (break))))

(fn `NextCharacter`
  (params (Swticher :type "/Game/Core/Blueprints/Characters/CharacterSelector/BP_CharacterSelection Object Reference"))
  (returns (SelectedCharacter :type "/Game/Core/Data/Enums/E_CharacterClasses Enum"))
  (`/Game/Core/Blueprints/Characters/CharacterSelector/BP_CharacterSelection.FlipAnimation` Swticher true)
  (switch `/Game/Core/Data/Enums/E_CharacterClasses` (`/Game/Core/Blueprints/Characters/CharacterSelector/BP_CharacterSelection.eCurrentCharacter` Swticher)
    (:`NewEnumerator0`
      (bind _output_get (set `/Game/Core/Blueprints/Characters/CharacterSelector/BP_CharacterSelection.eCurrentCharacter` "NewEnumerator1" Swticher))
      (return _output_get))
    (:`NewEnumerator1`
      (bind _output_get_2 (set `/Game/Core/Blueprints/Characters/CharacterSelector/BP_CharacterSelection.eCurrentCharacter` "NewEnumerator2" Swticher))
      (return _output_get_2))
    (:`NewEnumerator2`
      (bind _output_get_3 (set `/Game/Core/Blueprints/Characters/CharacterSelector/BP_CharacterSelection.eCurrentCharacter` "NewEnumerator0" Swticher))
      (return _output_get_3))))

(fn `OnRep_eSelectedCharacter`
  (`self.SetPlayerClass`))

(fn `OnRep_P1Locked?`
  (if (`self.P1Locked?`)
    (`/Game/Core/Blueprints/Functions/BFL_General.RemoveInputMappingContext` self "/Game/Core/Blueprints/Input/InputActionMappings/IMC_CharacterSelection.IMC_CharacterSelection")
    (`/Game/Core/Blueprints/Functions/BFL_General.AddInputMappingContext` self "/Game/Core/Blueprints/Input/InputActionMappings/IMC_Lock.IMC_Lock" 1)
    (else
      (`/Game/Core/Blueprints/Functions/BFL_General.RemoveInputMappingContext` self "/Game/Core/Blueprints/Input/InputActionMappings/IMC_Lock.IMC_Lock")
      (`/Game/Core/Blueprints/Functions/BFL_General.AddInputMappingContext` self "/Game/Core/Blueprints/Input/InputActionMappings/IMC_CharacterSelection.IMC_CharacterSelection" 1))))

(fn `OnRep_P2Locked?`
  (if (`self.P2Locked?`)
    (`/Game/Core/Blueprints/Functions/BFL_General.RemoveInputMappingContext` self "/Game/Core/Blueprints/Input/InputActionMappings/IMC_CharacterSelection.IMC_CharacterSelection")
    (`/Game/Core/Blueprints/Functions/BFL_General.AddInputMappingContext` self "/Game/Core/Blueprints/Input/InputActionMappings/IMC_Lock.IMC_Lock" 1)
    (else
      (`/Game/Core/Blueprints/Functions/BFL_General.RemoveInputMappingContext` self "/Game/Core/Blueprints/Input/InputActionMappings/IMC_Lock.IMC_Lock")
      (`/Game/Core/Blueprints/Functions/BFL_General.AddInputMappingContext` self "/Game/Core/Blueprints/Input/InputActionMappings/IMC_CharacterSelection.IMC_CharacterSelection" 1))))

(fn `PreviousCharacter`
  (params (Switcher :type "/Game/Core/Blueprints/Characters/CharacterSelector/BP_CharacterSelection Object Reference"))
  (returns (SelectedCharacter :type "/Game/Core/Data/Enums/E_CharacterClasses Enum"))
  (`/Game/Core/Blueprints/Characters/CharacterSelector/BP_CharacterSelection.FlipAnimation` Switcher false)
  (switch `/Game/Core/Data/Enums/E_CharacterClasses` (`/Game/Core/Blueprints/Characters/CharacterSelector/BP_CharacterSelection.eCurrentCharacter` Switcher)
    (:`NewEnumerator0`
      (bind _output_get (set `/Game/Core/Blueprints/Characters/CharacterSelector/BP_CharacterSelection.eCurrentCharacter` "NewEnumerator2" Switcher))
      (return _output_get))
    (:`NewEnumerator1`
      (bind _output_get_2 (set `/Game/Core/Blueprints/Characters/CharacterSelector/BP_CharacterSelection.eCurrentCharacter` "NewEnumerator0" Switcher))
      (return _output_get_2))
    (:`NewEnumerator2`
      (bind _output_get_3 (set `/Game/Core/Blueprints/Characters/CharacterSelector/BP_CharacterSelection.eCurrentCharacter` "NewEnumerator1" Switcher))
      (return _output_get_3))))

(fn `SelectArena`
  (`self.ChooseArena`)
  (if (`self.IsServer?`)
    (set `self.iIndex` 2)
    (`self.ResetGate`)))

(fn `StartGame`
  (bind _characterselectionref (`self.CharacterSelectionRef`))
  (`/Engine/EditorBlueprintResources/StandardMacros.IsValid` _characterselectionref
    (:`Is Valid`
      (`/Game/Core/Widgets/CharacterSelection/W_CharacterSelectionScreen.LockArena` _characterselectionref)
      (bind _outactors (`GameplayStatics.GetAllActorsOfClass` "/Game/Core/Blueprints/Characters/CharacterSelector/BP_CharacterSelection.BP_CharacterSelection_C"))
      (for _array_element _outactors
        (`/Game/Core/Blueprints/Characters/CharacterSelector/BP_CharacterSelection.FaceOffAnimation` _array_element))
      (`self.DisableInput` self))))

(fn `SwitchCharacter`
  (params (NextPrev :type Boolean) (`WhichPlayer?` :type "/Game/Core/Blueprints/Characters/CharacterSelector/BP_CharacterSelection Object Reference"))
  (if NextPrev
    (bind _selectedcharacter (`self.NextCharacter` `WhichPlayer?`))
    (set `self.eSelectedCharacter` _selectedcharacter)
    (else
      (bind _selectedcharacter_2 (`self.PreviousCharacter` `WhichPlayer?`))
      (set `self.eSelectedCharacter` _selectedcharacter_2))))

(fn `UserConstructionScript`)