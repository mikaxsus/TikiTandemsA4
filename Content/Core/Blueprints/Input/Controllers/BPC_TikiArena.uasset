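; Player controller for the online Tiki arena, covering spawning, input, loading screen, pause menu and end-game data.
; Server RPCs spawn the GameInstance-selected class, with team set by player-index parity, and multicast class, intro playback and skipping.
; OnRep PlayerClass picks the intro sequence by class-name substring; playback tints cinematic meshes by team and arena type.
; Enhanced Input forwards movement and combat to the possessed BP_Tiki, swapping mapping contexts on pause.
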(event `CL_SetHardQuit`
  (params (bQuit :type Boolean))
  (switch `/Game/Core/Data/Enums/E_Team` (`self.ePlayerTeam`)
    (:`NewEnumerator1`
      (bind _asgi_tiki_tandems (cast `/Game/Core/Blueprints/GameRules/GI_TikiTandems` (`GameplayStatics.GetGameInstance`)))
      (set `/Game/Core/Blueprints/GameRules/GI_TikiTandems.bQuit` bQuit _asgi_tiki_tandems))))

(event `SR_Spawn`
  (params (Class :type "/Game/Core/Blueprints/TikiCharacter/Blueprint/BP_Tiki Class Reference") (TeamTag :type Name))
  ;[1 1 1] Begin play
  (bind _asgm_arena (cast `/Game/Core/Blueprints/GameRules/GameModes/GM_Arena` (`GameplayStatics.GetGameMode`)))
  (`/Game/Core/Blueprints/GameRules/GameModes/GM_Arena.SpawnAndPossessPlayer` _asgm_arena self Class TeamTag)
  (`self.SetTeam`))

(event `MC_SetAnimationValues`
  (params (PlayerIndex :type Integer) (PlayerClass :type "/Game/Core/Blueprints/TikiCharacter/Blueprint/BP_Tiki Class Reference (by ref)"))
  ;[1 1 1] Begin play
  (bind _asgs_tiki_arena (cast `/Game/Core/Blueprints/GameRules/GameStates/GS_TikiArena` (`GameplayStatics.GetGameState`)))
  (`KismetArrayLibrary.Array_Set` (`/Game/Core/Blueprints/GameRules/GameStates/GS_TikiArena.PlayerClasses` _asgs_tiki_arena) PlayerIndex PlayerClass))

(event `SR_SetAnimationValues`
  (params (PlayerIndex :type Integer) (PlayerClass :type "/Game/Core/Blueprints/TikiCharacter/Blueprint/BP_Tiki Class Reference (by ref)"))
  ;[1 1 1] Begin play
  (`self.MC_SetAnimationValues` PlayerIndex PlayerClass))

(event `CL_SetEndGameStructs`
  (params (Winner :type "/Game/Core/Data/CharacterData/ST_EndInfo Structure") (Loser :type "/Game/Core/Data/CharacterData/ST_EndInfo Structure"))
  ;[1 1 1] SetEndGameCosmetic logic
  (bind _asgi_tiki_tandems (cast `/Game/Core/Blueprints/GameRules/GI_TikiTandems` (`GameplayStatics.GetGameInstance`)))
  (set `/Game/Core/Blueprints/GameRules/GI_TikiTandems.stWinnerInfo` Winner _asgi_tiki_tandems)
  (set `/Game/Core/Blueprints/GameRules/GI_TikiTandems.stLoserInfo` Loser _asgi_tiki_tandems))

(event `self.ReceiveBeginPlay`
  ;[1 1 1] Begin play
  (`self.CL_LoadingScreen`)
  (`KismetSystemLibrary.Delay` 0.2)
  (`self.SpawnCharacter`)
  (`KismetSystemLibrary.Delay` 0.2)
  (bind _asbp_tiki (cast `/Game/Core/Blueprints/TikiCharacter/Blueprint/BP_Tiki` (`self.K2_GetPawn`)))
  (set `self.BPTikiReference` _asbp_tiki)
  (`WidgetBlueprintLibrary.SetInputMode_GameOnly` self)
  (`self.CL_SetHardQuit` true))

(event `CL_CreateSkipButtonWidget`
  ;[1 1 1] Create/Remove skip button logic
  (bind _returnvalue (`|CreateWidget` "/Game/Core/Widgets/NewWidgets/W_SkipCinematic.W_SkipCinematic_C"))
  (bind _output_get (set `self.wSkipCinematic` _returnvalue))
  (`UserWidget.AddToViewport` _output_get 0)
  (set `self.bShowMouseCursor` true))

(event `CL_RemoveSkipButtonWidget`
  ;[1 1 1] Create/Remove skip button logic
  (`Widget.RemoveFromParent` (`self.wSkipCinematic`)))

(event `CL_LoadingScreen`
  ;[1 1 1] Show loading screen
  (bind _loadingscreenwidget (`/Game/Core/Blueprints/Functions/BFL_General.CreateLoadingScreen` self))
  (set `self.Loading Screen Widget` _loadingscreenwidget))

(event `EnhancedInput|/Game/Core/Blueprints/Input/InputActions/IA_BasicAttack`
  (params (ActionValue :type Boolean) (ElapsedSeconds :type "Float (double-precision)") (TriggeredSeconds :type "Float (double-precision)") (InputAction :type "InputAction Object Reference" :default "/Game/Core/Blueprints/Input/InputActions/IA_BasicAttack.IA_BasicAttack"))
  (bind _bptikireference (`self.BPTikiReference`))
  ;[1 1 1] Combat input
  (:`Triggered`
    (message `/Game/Core/Blueprints/Input/Interfaces/BPI_Combat.IC_BasicAttackTriggered` _bptikireference ElapsedSeconds))
  (:`Started`
    (message `/Game/Core/Blueprints/Input/Interfaces/BPI_Combat.IC_BasicAttackStarted` _bptikireference))
  (:`Completed`
    (message `/Game/Core/Blueprints/Input/Interfaces/BPI_Combat.IC_BasicAttackCompleted` _bptikireference)))

(event `EnhancedInput|/Game/Core/Blueprints/Input/InputActions/IA_Look`
  (params (ActionValue :type "Vector2D Structure") (ElapsedSeconds :type "Float (double-precision)") (TriggeredSeconds :type "Float (double-precision)") (InputAction :type "InputAction Object Reference" :default "/Game/Core/Blueprints/Input/InputActions/IA_Look.IA_Look"))
  ;[1 1 1] Basic input
  (:`Triggered`
    (`/Game/Core/Blueprints/TikiCharacter/Blueprint/BP_Tiki.LookInput` (`self.BPTikiReference`) ActionValue_X ActionValue_Y)))

(event `CL_RemoveLoadingScreen`
  ;[1 1 1] Show loading screen
  (`Widget.RemoveFromParent` (`self.Loading Screen Widget`)))

(event `SR_EndSequence`
  ;[1 1 1] End SequencePlayer Logic
  (`self.MC_EndSequence`))

(event `EnhancedInput|/Game/Core/Blueprints/Input/InputActions/IA_Move`
  (params (ActionValue :type "Vector2D Structure") (ElapsedSeconds :type "Float (double-precision)") (TriggeredSeconds :type "Float (double-precision)") (InputAction :type "InputAction Object Reference" :default "/Game/Core/Blueprints/Input/InputActions/IA_Move.IA_Move"))
  ;[1 1 1] Basic input
  (:`Triggered`
    (`/Game/Core/Blueprints/TikiCharacter/Blueprint/BP_Tiki.MoveInput` (`self.BPTikiReference`) ActionValue_X ActionValue_Y)))

(event `MC_EndSequence`
  (bind _activeplayersequence (`self.ActivePlayerSequence`))
  ;[1 1 1] End SequencePlayer Logic
  (`/Engine/EditorBlueprintResources/StandardMacros.IsValid` _activeplayersequence
    (:`Is Valid`
      (`MovieSceneSequencePlayer.GoToEndAndStop` _activeplayersequence)
      (`self.CL_RemoveSkipButtonWidget`))))

(event `EnhancedInput|/Game/Core/Blueprints/Input/InputActions/IA_SpecialAttack`
  (params (ActionValue :type Boolean) (ElapsedSeconds :type "Float (double-precision)") (TriggeredSeconds :type "Float (double-precision)") (InputAction :type "InputAction Object Reference" :default "/Game/Core/Blueprints/Input/InputActions/IA_SpecialAttack.IA_SpecialAttack"))
  ;[1 1 1] Combat input
  (:`Started`
    (message `/Game/Core/Blueprints/Input/Interfaces/BPI_Combat.IC_SpecialAttackStarted` (`self.BPTikiReference`))))

(event `EnhancedInput|/Game/Core/Blueprints/Input/InputActions/IA_Jump`
  (params (ActionValue :type Boolean) (ElapsedSeconds :type "Float (double-precision)") (TriggeredSeconds :type "Float (double-precision)") (InputAction :type "InputAction Object Reference" :default "/Game/Core/Blueprints/Input/InputActions/IA_Jump.IA_Jump"))
  ;[1 1 1] Basic input
  (:`Started`
    (`/Game/Core/Blueprints/TikiCharacter/Blueprint/BP_Tiki.JumpInput` (`self.BPTikiReference`))))

(event `EnhancedInput|/Game/Core/Blueprints/Input/InputActions/IA_HeavyAttack`
  (params (ActionValue :type Boolean) (ElapsedSeconds :type "Float (double-precision)") (TriggeredSeconds :type "Float (double-precision)") (InputAction :type "InputAction Object Reference" :default "/Game/Core/Blueprints/Input/InputActions/IA_HeavyAttack.IA_HeavyAttack"))
  ;[1 1 1] Combat input
  (:`Started`
    (message `/Game/Core/Blueprints/Input/Interfaces/BPI_Combat.IC_HeavyAttackStarted` (`self.BPTikiReference`))))

(event `CL_AddInputs`
  ;[1 1 1] Add input
  (`/Game/Core/Blueprints/Functions/BFL_General.AddInputMappingContext` self "/Game/Core/Blueprints/Input/InputActionMappings/IMC_Combat.IMC_Combat" 1)
  (`/Game/Core/Blueprints/TikiCharacter/Blueprint/BP_Tiki.CreateGameOverlay` (`self.BPTikiReference`))
  (bind _asgi_tiki_tandems (cast `/Game/Core/Blueprints/GameRules/GI_TikiTandems` (`GameplayStatics.GetGameInstance`)))
  (set `/Game/Core/Blueprints/GameRules/GI_TikiTandems.iPlayerIndex` (`self.iPlayerIndex`) _asgi_tiki_tandems)
  (set `self.bShowMouseCursor` false))

(event `EnhancedInput|/Game/Core/Blueprints/Input/InputActions/IA_Exit`
  (params (ActionValue :type Boolean) (ElapsedSeconds :type "Float (double-precision)") (TriggeredSeconds :type "Float (double-precision)") (InputAction :type "InputAction Object Reference" :default "/Game/Core/Blueprints/Input/InputActions/IA_Exit.IA_Exit"))
  ;[1 1 1] Combat input
  (:`Started`
    (`/Engine/EditorBlueprintResources/StandardMacros.FlipFlop`
      (:`A`
        (`self.PauseGame`))
      (:`B`
        (`self.ResumeGame`)))))

(event `PauseGame`
  ;[1 1 1] Pause/Resume logic
  (bind _returnvalue (`|CreateWidget` "/Game/Core/Widgets/NewWidgets/W_PauseMenu.W_PauseMenu_C" self))
  (bind _output_get (set `self.wPauseMenu` _returnvalue))
  (`UserWidget.AddToViewport` _output_get 0)
  (`WidgetBlueprintLibrary.SetInputMode_GameAndUIEx` self null)
  (set `self.bShowMouseCursor` true)
  (`/Game/Core/Blueprints/Functions/BFL_General.AddInputMappingContext` self "/Game/Core/Blueprints/Input/InputActionMappings/IMC_Exit.IMC_Exit" 1)
  (`/Game/Core/Blueprints/Functions/BFL_General.RemoveInputMappingContext` self "/Game/Core/Blueprints/Input/InputActionMappings/IMC_Combat.IMC_Combat"))

(event `SR_PlayAnimation`
  (params (PlayerClass :type "/Game/Core/Blueprints/TikiCharacter/Blueprint/BP_Tiki Class Reference") (PlayerIndex :type Integer))
  ;[1 1 1] PlaySequence logic
  (`self.MC_PlayAnimation` PlayerClass PlayerIndex))

(event `Key|AnyKey`
  (params (Key :type "Key Structure"))
  (bind _wskipcinematic (`self.wSkipCinematic`))
  ;[1 1 1] Mouse cursor show/hide logic
  (:`Pressed`
    (if (`KismetInputLibrary.Key_IsGamepadKey` Key)
      (`/Engine/EditorBlueprintResources/StandardMacros.IsValid` _wskipcinematic
        (:`Is Valid`
          (`Widget.SetFocus` (`/Game/Core/Widgets/NewWidgets/W_SkipCinematic.W_CustomButton` _wskipcinematic))
          (set `self.bShowMouseCursor` false)))
      (else
        (`WidgetBlueprintLibrary.SetFocusToGameViewport`)))))

(event `MC_PlayAnimation`
  (params (PlayerClass :type "/Game/Core/Blueprints/TikiCharacter/Blueprint/BP_Tiki Class Reference") (PlayerIndex :type Integer))
  ;[1 1 1] PlaySequence logic
  (`self.PlayAnimation` PlayerClass PlayerIndex))

(event `ResumeGame`
  ;[1 1 1] Pause/Resume logic
  (`Widget.RemoveFromParent` (`self.wPauseMenu`))
  (`WidgetBlueprintLibrary.SetInputMode_GameOnly` self)
  (set `self.bShowMouseCursor` false)
  (`WidgetBlueprintLibrary.SetFocusToGameViewport`)
  (`/Game/Core/Blueprints/Functions/BFL_General.AddInputMappingContext` self "/Game/Core/Blueprints/Input/InputActionMappings/IMC_Combat.IMC_Combat" 1)
  (`/Game/Core/Blueprints/Functions/BFL_General.RemoveInputMappingContext` self "/Game/Core/Blueprints/Input/InputActionMappings/IMC_Exit.IMC_Exit"))

(fn `OnRep_PlayerClass`
  (`self.SwitchOnBP_TikiClass` (`self.PlayerClass`)))

(fn `PlayAnimation`
  (params (PlayerClass :type "/Game/Core/Blueprints/TikiCharacter/Blueprint/BP_Tiki Class Reference") (PlayerIndex :type Integer))
  (locals (L_SequenceSettings :type "MovieSceneSequencePlaybackSettings Structure" :default (struct :`LoopCount` (struct) :`TickInterval` (struct :`bAllowRounding` true) :`PlayRate` 1.0 :`bRestoreState` true :`bInheritTickIntervalFromOwner` true)) (L_LevelSequenceActor :type "LevelSequenceActor Object Reference") (L_Counter :type Integer))
  (set `self.PlayerClass` PlayerClass)
  (`|ExecutionSequence`
    (:`then_0`
      (bind _asgi_tiki_tandems (cast `/Game/Core/Blueprints/GameRules/GI_TikiTandems` (`GameplayStatics.GetGameInstance`)))
      (bind _outactors (`GameplayStatics.GetAllActorsOfClassWithTag` "/Script/Engine.SkeletalMeshActor" "Cinematic"))
      (for _array_element _outactors
        (if (== (mod PlayerIndex 2) 0)
          (bind _earenatype (`/Game/Core/Blueprints/GameRules/GI_TikiTandems.eArenaType` _asgi_tiki_tandems))
          (switch `/Game/Core/Data/Enums/E_ArenaType` _earenatype
            (:`NewEnumerator0`
              (bind _skeletalmeshcomponent (`SkeletalMeshActor.SkeletalMeshComponent` _array_element))
              (`MeshComponent.SetOverlayMaterial` _skeletalmeshcomponent "/Game/Assets/TikiCharacter/Materials/MI_RedPlayer.MI_RedPlayer"))
            (:`NewEnumerator1`
              (`MeshComponent.SetOverlayMaterial` _skeletalmeshcomponent "/Game/Assets/TikiCharacter/Materials/MI_PurplePLayer.MI_PurplePLayer")))
          (else
            (switch `/Game/Core/Data/Enums/E_ArenaType` _earenatype
              (:`NewEnumerator0`
                (`MeshComponent.SetOverlayMaterial` _skeletalmeshcomponent "/Game/Assets/TikiCharacter/Materials/MI_BluePlayer.MI_BluePlayer"))
              (:`NewEnumerator1`
                (`MeshComponent.SetOverlayMaterial` _skeletalmeshcomponent "/Game/Assets/TikiCharacter/Materials/MI_YellowPlayer.MI_YellowPlayer")))))))
    (:`then_1`
      (bind _outactor (`LevelSequencePlayer.CreateLevelSequencePlayer` (`self.ActiveLevelSequence`) (`local.L_SequenceSettings`)))
      (bind _output_get (set `local.L_LevelSequenceActor` _outactor))
      (`MovieSceneSequencePlayer.Play` (`LevelSequenceActor.SequencePlayer` _outactor))
      (set `self.ActivePlayerSequence` (`LevelSequenceActor.SequencePlayer` _output_get)))
    (:`then_2`
      (return))))

(fn `SetQuitLogic`
  (params (PlayerClasses :type "Array of /Game/Core/Blueprints/TikiCharacter/Blueprint/BP_Tiki Class Reference"))
  (bind _asgi_tiki_tandems (cast `/Game/Core/Blueprints/GameRules/GI_TikiTandems` (`GameplayStatics.GetGameInstance`)))
  (for (_array_element _array_index) PlayerClasses
    (bind _playerclasses (`/Game/Core/Blueprints/GameRules/GI_TikiTandems.PlayerClasses` _asgi_tiki_tandems))
    (`KismetArrayLibrary.Array_Set` _playerclasses _array_index _array_element true))
  (for (_array_element_2 _array_index_2) _playerclasses
    (if (== (mod _array_index_2 2) 0)
      (bind _stplayers (`/Game/Core/Blueprints/GameRules/GI_TikiTandems.stPlayers` _asgi_tiki_tandems))
      (`KismetArrayLibrary.Array_Set` _stplayers _array_index_2 (make `/Game/Core/Data/CharacterData/ST_EndInfo` _array_element_2) true)
      (else
        (`KismetArrayLibrary.Array_Set` _stplayers _array_index_2 (make `/Game/Core/Data/CharacterData/ST_EndInfo` _array_element_2 "NewEnumerator1") true))))
  (bind (_output_characterclass _output_playerteam) (break `/Game/Core/Data/CharacterData/ST_EndInfo` (`|GetArrayItem` _stplayers)))
  (bind (_output_characterclass_2 _output_playerteam_2) (break `/Game/Core/Data/CharacterData/ST_EndInfo` (`|GetArrayItem` _stplayers 1)))
  (`KismetSystemLibrary.PrintString` (`KismetStringLibrary.Concat_StrStr` (`KismetSystemLibrary.GetClassDisplayName` _output_characterclass) " " (`|GetEnumeratorNameAsString` _output_playerteam) (`KismetSystemLibrary.GetClassDisplayName` _output_characterclass_2) " " (`|GetEnumeratorNameAsString` _output_playerteam_2)) true true (struct :`G` 0.66 :`B` 1.0 :`A` 1.0) 20.0))

(fn `SetTeam`
  (if (== (mod (`self.iPlayerIndex`) 2) 0)
    (set `self.ePlayerTeam` "NewEnumerator0")
    (else
      (set `self.ePlayerTeam` "NewEnumerator1"))))

(fn `SpawnCharacter`
  (bind _iplayerindex (`self.iPlayerIndex`))
  (bind _asgi_tiki_tandems (cast `/Game/Core/Blueprints/GameRules/GI_TikiTandems` (`GameplayStatics.GetGameInstance`)))
  (if (== (mod _iplayerindex 2) 0)
    (bind _playerclass (`/Game/Core/Blueprints/GameRules/GI_TikiTandems.PlayerClass` _asgi_tiki_tandems))
    (`self.SR_Spawn` _playerclass "Red")
    (else
      (`self.SR_Spawn` _playerclass "Blue")))
  (`self.SR_SetAnimationValues` _iplayerindex _playerclass))

(fn `UserConstructionScript`)