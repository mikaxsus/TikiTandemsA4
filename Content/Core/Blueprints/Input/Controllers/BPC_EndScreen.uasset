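; BPC_EndScreen is the player controller for the end screen, covering it with a loading screen on BeginPlay.
; A client loading-screen removal event swaps that widget for W_WinScreen and shows the cursor.
; Gamepad presses focus the win screen's Quick button and hide the cursor; other keys return focus to the viewport.
; QuitGame waits briefly, destroys EIK sessions and opens L_MainMenu, while NewQuickGame is an empty stub.
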(event `self.ReceiveBeginPlay`
  ;[1 1 1] EventBeginPlay
  (`self.CL_CreateLoadingScreen`))

(event `CL_CreateLoadingScreen`
  ;[1 1 1] Create/Destroy loading screen
  (bind _loadingscreenwidget (`/Game/Core/Blueprints/Functions/BFL_General.CreateLoadingScreen` self))
  (set `self.wLoadingScreen` _loadingscreenwidget))

(event `CL_RemoveLoadingScreen`
  ;[1 1 1] Create/Destroy loading screen
  (`Widget.RemoveFromParent` (`self.wLoadingScreen`))
  (bind _returnvalue (`|CreateWidget` "/Game/Core/Widgets/MainMenu/W_WinScreen.W_WinScreen_C"))
  (bind _output_get (set `self.wWinScreen` _returnvalue))
  (`UserWidget.AddToViewport` _output_get 0)
  (set `self.bShowMouseCursor` true))

(event `Key|AnyKey`
  (params (Key :type "Key Structure"))
  (bind _wwinscreen (`self.wWinScreen`))
  ;[1 1 1] Set focus to one button
  (:`Pressed`
    (if (`KismetInputLibrary.Key_IsGamepadKey` Key)
      (`/Engine/EditorBlueprintResources/StandardMacros.IsValid` _wwinscreen
        (:`Is Valid`
          (`Widget.SetFocus` (`/Game/Core/Widgets/MainMenu/W_WinScreen.Quick` _wwinscreen))
          (set `self.bShowMouseCursor` false)))
      (else
        (`WidgetBlueprintLibrary.SetFocusToGameViewport`)))))

(event `QuitGame`
  ;[1 1 1] Widget logic
  (`KismetSystemLibrary.Delay` 2.0)
  (`EIK_DestroySession_AsyncFunction.DestroyEIKSessions` (struct)
    (:`then`
      (`GameplayStatics.OpenLevelBySoftObjectPtr` "/Game/maps/L_MainMenu.L_MainMenu"))))

(event `NewQuickGame`
  ;[1 1 1] Widget logic
)

(fn `UserConstructionScript`)