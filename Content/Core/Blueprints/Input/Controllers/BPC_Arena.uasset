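; BPC_Arena is the arena player controller that routes Enhanced Input actions to the controlled BP_Tiki pawn.
; On BeginPlay it adds the IMC_Combat mapping context and caches a cast reference to the pawn.
; Look, Move and Jump forward to the pawn's input functions, while Basic, Heavy and Special attacks only print debug strings.
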(event `self.ReceiveBeginPlay`
  ;[1 1 1] Begin play
  (`/Game/Core/Blueprints/Functions/BFL_General.AddInputMappingContext` self "/Game/Core/Blueprints/Input/InputActionMappings/IMC_Combat.IMC_Combat")
  (bind _asbp_tiki (cast `/Game/Core/Blueprints/TikiCharacter/Blueprint/BP_Tiki` (`self.K2_GetPawn`)))
  (set `self.BPTikiReference` _asbp_tiki))

(event `EnhancedInput|/Game/Core/Blueprints/Input/InputActions/IA_BasicAttack`
  (params (ActionValue :type Boolean) (ElapsedSeconds :type "Float (double-precision)") (TriggeredSeconds :type "Float (double-precision)") (InputAction :type "InputAction Object Reference" :default "/Game/Core/Blueprints/Input/InputActions/IA_BasicAttack.IA_BasicAttack"))
  ;[1 1 1] Combat input
  (:`Triggered`
    (`KismetSystemLibrary.PrintString` "BasicAttack")))

(event `EnhancedInput|/Game/Core/Blueprints/Input/InputActions/IA_Look`
  (params (ActionValue :type "Vector2D Structure") (ElapsedSeconds :type "Float (double-precision)") (TriggeredSeconds :type "Float (double-precision)") (InputAction :type "InputAction Object Reference" :default "/Game/Core/Blueprints/Input/InputActions/IA_Look.IA_Look"))
  ;[1 1 1] Basic input
  (:`Triggered`
    (`/Game/Core/Blueprints/TikiCharacter/Blueprint/BP_Tiki.LookInput` (`self.BPTikiReference`) ActionValue_X ActionValue_Y)))

(event `EnhancedInput|/Game/Core/Blueprints/Input/InputActions/IA_SpecialAttack`
  (params (ActionValue :type Boolean) (ElapsedSeconds :type "Float (double-precision)") (TriggeredSeconds :type "Float (double-precision)") (InputAction :type "InputAction Object Reference" :default "/Game/Core/Blueprints/Input/InputActions/IA_SpecialAttack.IA_SpecialAttack"))
  ;[1 1 1] Combat input
  (:`Triggered`
    (`KismetSystemLibrary.PrintString` "SpecialAttack")))

(event `EnhancedInput|/Game/Core/Blueprints/Input/InputActions/IA_Move`
  (params (ActionValue :type "Vector2D Structure") (ElapsedSeconds :type "Float (double-precision)") (TriggeredSeconds :type "Float (double-precision)") (InputAction :type "InputAction Object Reference" :default "/Game/Core/Blueprints/Input/InputActions/IA_Move.IA_Move"))
  ;[1 1 1] Basic input
  (:`Triggered`
    (`/Game/Core/Blueprints/TikiCharacter/Blueprint/BP_Tiki.MoveInput` (`self.BPTikiReference`) ActionValue_X ActionValue_Y)))

(event `EnhancedInput|/Game/Core/Blueprints/Input/InputActions/IA_HeavyAttack`
  (params (ActionValue :type Boolean) (ElapsedSeconds :type "Float (double-precision)") (TriggeredSeconds :type "Float (double-precision)") (InputAction :type "InputAction Object Reference" :default "/Game/Core/Blueprints/Input/InputActions/IA_HeavyAttack.IA_HeavyAttack"))
  ;[1 1 1] Combat input
  (:`Triggered`
    (`KismetSystemLibrary.PrintString` "HeavyAttack")))

(event `EnhancedInput|/Game/Core/Blueprints/Input/InputActions/IA_Jump`
  (params (ActionValue :type Boolean) (ElapsedSeconds :type "Float (double-precision)") (TriggeredSeconds :type "Float (double-precision)") (InputAction :type "InputAction Object Reference" :default "/Game/Core/Blueprints/Input/InputActions/IA_Jump.IA_Jump"))
  ;[1 1 1] Basic input
  (:`Started`
    (`/Game/Core/Blueprints/TikiCharacter/Blueprint/BP_Tiki.JumpInput` (`self.BPTikiReference`))))

(fn `UserConstructionScript`)