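; Local-play player controller for the Tiki arena, handling each player's intro cinematic, combat input, HUD and pause menu.
; PlayAnimation picks a Level Sequence by class-name substring, tints cinematic meshes by player parity and arena type, and applies a view-flip post-process for odd players.
; AddInputs caches the BP_Tiki pawn that receives forwarded input, creates the HUD and assigns team by index parity.
; IA_Exit toggles the pause menu, swapping combat and exit mapping contexts.
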(event `CreateOverlay`
  ;[1 1 1] Create UI
  (bind _returnvalue (`|CreateWidget` "/Game/Core/Widgets/NewHUDs/W_CharacterOverlay_Local.W_CharacterOverlay_Local_C" self))
  (bind _output_get (set `self.HUD` _returnvalue))
  (`UserWidget.AddToPlayerScreen` _output_get 0))

(event `AddInputs`
  ;[1 1 1] Add input
  (`/Game/Core/Blueprints/Functions/BFL_General.AddInputMappingContext` self "/Game/Core/Blueprints/Input/InputActionMappings/IMC_Combat.IMC_Combat")
  (`KismetSystemLibrary.Delay` 0.2)
  (bind _asbp_tiki (cast `/Game/Core/Blueprints/TikiCharacter/Blueprint/BP_Tiki` (`self.K2_GetPawn`)))
  (set `self.BPTikiReference` _asbp_tiki)
  (`WidgetBlueprintLibrary.SetInputMode_GameOnly` self)
  (`self.CreateOverlay`)
  (`self.RemoveSkipButtonWidget`)
  (`self.SetTeam`))

(event `EnhancedInput|/Game/Core/Blueprints/Input/InputActions/IA_BasicAttack`
  (params (ActionValue :type Boolean) (ElapsedSeconds :type "Float (double-precision)") (TriggeredSeconds :type "Float (double-precision)") (InputAction :type "InputAction Object Reference" :default "/Game/Core/Blueprints/Input/InputActions/IA_BasicAttack.IA_BasicAttack"))
  (bind _bptikireference (`self.BPTikiReference`))
  ;[1 1 1] Combat input
  (:`Triggered`
    (message `/Game/Core/Blueprints/Input/Interfaces/BPI_Combat.IC_BasicAttackTriggered` _bptikireference ElapsedSeconds))
  (:`Started`
    (message `/Game/Core/Blueprints/Input/Interfaces/BPI_Combat.IC_BasicAttackStarted` _bptikireference))
  (:`Completed`
    (message `/Game/Core/Blueprints/Input/Interfaces/BPI_Combat.IC_BasicAttackCompleted` _bptikireference)))

(event `EnhancedInput|/Game/Core/Blueprints/Input/InputActions/IA_Look`
  (params (ActionValue :type "Vector2D Structure") (ElapsedSeconds :type "Float (double-precision)") (TriggeredSeconds :type "Float (double-precision)") (InputAction :type "InputAction Object Reference" :default "/Game/Core/Blueprints/Input/InputActions/IA_Look.IA_Look"))
  ;[1 1 1] Basic input
  (:`Triggered`
    (`/Game/Core/Blueprints/TikiCharacter/Blueprint/BP_Tiki.LookInput` (`self.BPTikiReference`) ActionValue_X ActionValue_Y)))

(event `CreateSkipButtonWidget`
  ;[1 1 1] Create/Remove skip button logic
  (bind _returnvalue (`|CreateWidget` "/Game/Core/Widgets/NewWidgets/W_SkipCinematic.W_SkipCinematic_C"))
  (bind _output_get (set `self.wSkipCinematic` _returnvalue))
  (`UserWidget.AddToViewport` _output_get 0)
  (set `self.bShowMouseCursor` true))

(event `EnhancedInput|/Game/Core/Blueprints/Input/InputActions/IA_Move`
  (params (ActionValue :type "Vector2D Structure") (ElapsedSeconds :type "Float (double-precision)") (TriggeredSeconds :type "Float (double-precision)") (InputAction :type "InputAction Object Reference" :default "/Game/Core/Blueprints/Input/InputActions/IA_Move.IA_Move"))
  ;[1 1 1] Basic input
  (:`Triggered`
    (`/Game/Core/Blueprints/TikiCharacter/Blueprint/BP_Tiki.MoveInput` (`self.BPTikiReference`) ActionValue_X ActionValue_Y)))

(event `RemoveSkipButtonWidget`
  ;[1 1 1] Create/Remove skip button logic
  (`Widget.RemoveFromParent` (`self.wSkipCinematic`))
  (set `self.bShowMouseCursor` false))

(event `EnhancedInput|/Game/Core/Blueprints/Input/InputActions/IA_SpecialAttack`
  (params (ActionValue :type Boolean) (ElapsedSeconds :type "Float (double-precision)") (TriggeredSeconds :type "Float (double-precision)") (InputAction :type "InputAction Object Reference" :default "/Game/Core/Blueprints/Input/InputActions/IA_SpecialAttack.IA_SpecialAttack"))
  ;[1 1 1] Combat input
  (:`Started`
    (message `/Game/Core/Blueprints/Input/Interfaces/BPI_Combat.IC_SpecialAttackStarted` (`self.BPTikiReference`))))

(event `EnhancedInput|/Game/Core/Blueprints/Input/InputActions/IA_Jump`
  (params (ActionValue :type Boolean) (ElapsedSeconds :type "Float (double-precision)") (TriggeredSeconds :type "Float (double-precision)") (InputAction :type "InputAction Object Reference" :default "/Game/Core/Blueprints/Input/InputActions/IA_Jump.IA_Jump"))
  ;[1 1 1] Basic input
  (:`Started`
    (`/Game/Core/Blueprints/TikiCharacter/Blueprint/BP_Tiki.JumpInput` (`self.BPTikiReference`))))

(event `EnhancedInput|/Game/Core/Blueprints/Input/InputActions/IA_HeavyAttack`
  (params (ActionValue :type Boolean) (ElapsedSeconds :type "Float (double-precision)") (TriggeredSeconds :type "Float (double-precision)") (InputAction :type "InputAction Object Reference" :default "/Game/Core/Blueprints/Input/InputActions/IA_HeavyAttack.IA_HeavyAttack"))
  ;[1 1 1] Combat input
  (:`Started`
    (message `/Game/Core/Blueprints/Input/Interfaces/BPI_Combat.IC_HeavyAttackStarted` (`self.BPTikiReference`))))

(event `EndSequence`
  (bind _activeplayersequence (`self.ActivePlayerSequence`))
  ;[1 1 1] End SequencePlayer Logic
  (`/Engine/EditorBlueprintResources/StandardMacros.IsValid` _activeplayersequence
    (:`Is Valid`
      (`MovieSceneSequencePlayer.GoToEndAndStop` _activeplayersequence)
      (`self.RemoveSkipButtonWidget`))))

(event `EnhancedInput|/Game/Core/Blueprints/Input/InputActions/IA_Exit`
  (params (ActionValue :type Boolean) (ElapsedSeconds :type "Float (double-precision)") (TriggeredSeconds :type "Float (double-precision)") (InputAction :type "InputAction Object Reference" :default "/Game/Core/Blueprints/Input/InputActions/IA_Exit.IA_Exit"))
  ;[1 1 1] Combat input
  (:`Started`
    (`/Engine/EditorBlueprintResources/StandardMacros.FlipFlop`
      (:`A`
        (`self.PauseGame`))
      (:`B`
        (`self.ResumeGame`)))))

(event `PauseGame`
  ;[1 1 1] Pause/Resume logic
  (bind _returnvalue (`|CreateWidget` "/Game/Core/Widgets/NewWidgets/W_PauseMenu.W_PauseMenu_C" self))
  (bind _output_get (set `self.wPauseMenu` _returnvalue))
  (`UserWidget.AddToViewport` _output_get 0)
  (`WidgetBlueprintLibrary.SetInputMode_GameAndUIEx` self null)
  (set `self.bShowMouseCursor` true)
  (`/Game/Core/Blueprints/Functions/BFL_General.AddInputMappingContext` self "/Game/Core/Blueprints/Input/InputActionMappings/IMC_Exit.IMC_Exit")
  (`/Game/Core/Blueprints/Functions/BFL_General.RemoveInputMappingContext` self "/Game/Core/Blueprints/Input/InputActionMappings/IMC_Combat.IMC_Combat"))

(event `ResumeGame`
  ;[1 1 1] Pause/Resume logic
  (`Widget.RemoveFromParent` (`self.wPauseMenu`))
  (`WidgetBlueprintLibrary.SetInputMode_GameOnly` self)
  (set `self.bShowMouseCursor` false)
  (`WidgetBlueprintLibrary.SetFocusToGameViewport`)
  (`/Game/Core/Blueprints/Functions/BFL_General.AddInputMappingContext` self "/Game/Core/Blueprints/Input/InputActionMappings/IMC_Combat.IMC_Combat")
  (`/Game/Core/Blueprints/Functions/BFL_General.RemoveInputMappingContext` self "/Game/Core/Blueprints/Input/InputActionMappings/IMC_Exit.IMC_Exit"))

(fn `PlayAnimation`
  (params (PlayerClass :type "/Game/Core/Blueprints/TikiCharacter/Blueprint/BP_Tiki Class Reference") (PlayerIndex :type Integer))
  (locals (L_SequenceSettings :type "MovieSceneSequencePlaybackSettings Structure" :default (struct :`LoopCount` (struct) :`TickInterval` (struct :`bAllowRounding` true) :`PlayRate` 1.0 :`bRestoreState` true :`bInheritTickIntervalFromOwner` true)) (L_LevelSequenceActor :type "LevelSequenceActor Object Reference") (L_Counter :type Integer))
  (bind _output_get (set `self.PlayerClass` PlayerClass))
  (`self.SwitchOnBP_TikiClass` _output_get)
  (`|ExecutionSequence`
    (:`then_0`
      (bind _asgi_tiki_tandems (cast `/Game/Core/Blueprints/GameRules/GI_TikiTandems` (`GameplayStatics.GetGameInstance`)))
      (bind _outactors (`GameplayStatics.GetAllActorsOfClassWithTag` "/Script/Engine.SkeletalMeshActor" "Cinematic"))
      (for _array_element _outactors
        (if (== (mod PlayerIndex 2) 0)
          (bind _earenatype (`/Game/Core/Blueprints/GameRules/GI_TikiTandems.eArenaType` _asgi_tiki_tandems))
          (switch `/Game/Core/Data/Enums/E_ArenaType` _earenatype
            (:`NewEnumerator0`
              (bind _skeletalmeshcomponent (`SkeletalMeshActor.SkeletalMeshComponent` _array_element))
              (`MeshComponent.SetOverlayMaterial` _skeletalmeshcomponent "/Game/Assets/TikiCharacter/Materials/MI_RedPlayer.MI_RedPlayer"))
            (:`NewEnumerator1`
              (`MeshComponent.SetOverlayMaterial` _skeletalmeshcomponent "/Game/Assets/TikiCharacter/Materials/MI_PurplePLayer.MI_PurplePLayer")))
          (else
            (switch `/Game/Core/Data/Enums/E_ArenaType` _earenatype
              (:`NewEnumerator0`
                (`MeshComponent.SetOverlayMaterial` _skeletalmeshcomponent "/Game/Assets/TikiCharacter/Materials/MI_BluePlayer.MI_BluePlayer"))
              (:`NewEnumerator1`
                (`MeshComponent.SetOverlayMaterial` _skeletalmeshcomponent "/Game/Assets/TikiCharacter/Materials/MI_YellowPlayer.MI_YellowPlayer")))))))
    (:`then_1`
      (bind _outactor (`LevelSequencePlayer.CreateLevelSequencePlayer` (`self.ActiveLevelSequence`) (`local.L_SequenceSettings`)))
      (bind _output_get_2 (set `local.L_LevelSequenceActor` _outactor))
      (`MovieSceneSequencePlayer.Play` (`LevelSequenceActor.SequencePlayer` _outactor))
      (bind _sequenceplayer (`LevelSequenceActor.SequencePlayer` _output_get_2))
      (set `self.ActivePlayerSequence` _sequenceplayer)
      (if (not (== (mod PlayerIndex 2) 0))
        (bind _returnvalue (`KismetMaterialLibrary.CreateDynamicMaterialInstance` "/Game/Assets/UI/Materials/M_FlipView.M_FlipView"))
        (setmembers `PostProcessSettings` :`StructRef` (`CameraComponent.PostProcessSettings` (`LevelSequencePlayer.GetActiveCameraComponent` _sequenceplayer)) :`WeightedBlendables` (make `WeightedBlendables` (`|MakeArray` (make `WeightedBlendable` 1.0 _returnvalue))))))
    (:`then_2`
      (return))))

(fn `SetTeam`
  (if (== (mod (`self.iPlayerIndex`) 2) 0)
    (set `self.ePlayerTeam` "NewEnumerator0")
    (else
      (set `self.ePlayerTeam` "NewEnumerator1"))))

(fn `UserConstructionScript`)