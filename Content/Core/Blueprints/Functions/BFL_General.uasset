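; General Blueprint function library for Tiki Tandems, providing shared helpers for Enhanced Input and settings saving.
; Input helpers add, remove or clear mapping contexts on a player controller's local player subsystem, with validity checks on add and remove only.
; Settings helpers read the save object and slot name from GI_TikiTandems, then write that object to its slot.
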(fn `AddInputMappingContext`
  (params (PlayerController :type "PlayerController Object Reference") (MappingContext :type "InputMappingContext Object Reference") (Priority :type Integer))
  (bind _returnvalue (pcsubsystem `EnhancedInputLocalPlayerSubsystem` PlayerController))
  (`/Engine/EditorBlueprintResources/StandardMacros.IsValid` _returnvalue
    (:`Is Valid`
      (`EnhancedInputSubsystemInterface.AddMappingContext` _returnvalue MappingContext Priority (struct)))))

(fn `GetSettingsSave`
  (returns (`Settings Save` :type "/Game/Core/Blueprints/SaveGame/BP_SaveGameSettings Object Reference") (`Settings Slot` :type String))
  (bind _asgi_tiki_tandems (cast `/Game/Core/Blueprints/GameRules/GI_TikiTandems` (`GameplayStatics.GetGameInstance` null)))
  (return (`/Game/Core/Blueprints/GameRules/GI_TikiTandems.Settings Save` _asgi_tiki_tandems) (`/Game/Core/Blueprints/GameRules/GI_TikiTandems.Settings Slot` _asgi_tiki_tandems)))

(fn `RemoveAllInputMappingContexts`
  (params (PlayerController :type "PlayerController Object Reference"))
  (`EnhancedInputSubsystemInterface.ClearAllMappings` (pcsubsystem `EnhancedInputLocalPlayerSubsystem` PlayerController)))

(fn `RemoveInputMappingContext`
  (params (PlayerController :type "PlayerController Object Reference") (MappingContext :type "InputMappingContext Object Reference"))
  (bind _returnvalue (pcsubsystem `EnhancedInputLocalPlayerSubsystem` PlayerController))
  (`/Engine/EditorBlueprintResources/StandardMacros.IsValid` _returnvalue
    (:`Is Valid`
      (`EnhancedInputSubsystemInterface.RemoveMappingContext` _returnvalue MappingContext (struct)))))

(fn `SaveGameSettings`
  (bind (_settings_save _settings_slot) (`self.GetSettingsSave` null))
  (`GameplayStatics.SaveGameToSlot` _settings_save _settings_slot))