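; BP_Gate is a cinematic gate whose spears break apart with physics in two stages.
; Looping timers poll the BreakSpears flag, which is not set true in this graph.
; Each break simulates physics on three spears, adds a radial force at the Arrow, then destroys them after a delay.
; The first break reveals the second spear set, whose poll stops on trigger or after a timeout.
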(event `self.ReceiveBeginPlay`
  (bind _returnvalue (`KismetSystemLibrary.K2_SetTimerDelegate` (delegate `CheckSpearBreakage`) 0.05 true)))

(event `CheckSpearBreakage`
  (bind _spearmiddle2 (`self.SpearMiddle2`))
  (if (`self.BreakSpears?`)
    (`KismetSystemLibrary.K2_ClearAndInvalidateTimerHandle` (stale `self.ReceiveBeginPlay` _returnvalue))
    (`PrimitiveComponent.SetSimulatePhysics` _spearmiddle2 true)
    (`PrimitiveComponent.SetSimulatePhysics` (`self.SpearMiddle`) true)
    (`PrimitiveComponent.SetSimulatePhysics` (`self.SpearMiddle1`) true)
    (`AddComponent|NODE_AddRadialForceComponent-0` :`RelativeTransform` (`SceneComponent.GetRelativeTransform` (`self.Arrow`)))
    (`KismetSystemLibrary.Delay` 5.7)
    (`ActorComponent.K2_DestroyComponent` _spearmiddle2)
    (`ActorComponent.K2_DestroyComponent` (`self.SpearMiddle`))
    (`ActorComponent.K2_DestroyComponent` (`self.SpearMiddle1`))
    (`SceneComponent.SetHiddenInGame` (`self.SpearMiddle3`) false false)
    (`SceneComponent.SetHiddenInGame` (`self.SpearMiddle5`) false false)
    (`SceneComponent.SetHiddenInGame` (`self.SpearMiddle4`) false false)
    (bind _returnvalue (`KismetSystemLibrary.K2_SetTimerDelegate` (delegate `SecondBonkermanAnim`) 0.05 true))
    (set `self.BreakSpears?` false)))

(event `SecondBonkermanAnim`
  (if (`self.BreakSpears?`)
    (`KismetSystemLibrary.K2_ClearAndInvalidateTimerHandle` (stale `CheckSpearBreakage` _returnvalue))
    (`PrimitiveComponent.SetSimulatePhysics` (`self.SpearMiddle4`) true)
    (`PrimitiveComponent.SetSimulatePhysics` (`self.SpearMiddle5`) true)
    (`PrimitiveComponent.SetSimulatePhysics` (`self.SpearMiddle3`) true)
    (`AddComponent|NODE_AddRadialForceComponent-2` :`RelativeTransform` (`SceneComponent.GetRelativeTransform` (`self.Arrow`)))
    (`KismetSystemLibrary.Delay` 5.0)
    (`ActorComponent.K2_DestroyComponent` (`self.SpearMiddle3`))
    (`ActorComponent.K2_DestroyComponent` (`self.SpearMiddle5`))
    (`ActorComponent.K2_DestroyComponent` (`self.SpearMiddle4`))
    (else
      (`KismetSystemLibrary.Delay` 6.0)
      (`KismetSystemLibrary.K2_ClearAndInvalidateTimerHandle` (stale `CheckSpearBreakage` _returnvalue)))))

(fn `UserConstructionScript`)